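; AssessMetaPawn is the player pawn for a metamorphopsia eye test, where input adjusts a simulated scotoma per eye on a distortion plane.
; On BeginPlay it resolves nested child actors to reach the MetaCamera, its left and right UI widgets and the MetamorphopsiaController, then applies the PicoEye input mapping.
; Pico actions and debug keys drive eye, layer and property changes, plane toggling, and saving patient data before returning to EyeTests.
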(event Input|EnhancedActionEvents|EnhancedInputActionPicoInput8
  (params (ActionValue :type Vector%202D%20Structure) (ElapsedSeconds :type Float%20%28double-precision%29) (TriggeredSeconds :type Float%20%28double-precision%29) (InputAction :type Input%20Action%20Object%20Reference :default "/Game/PicoInput/PicoInput8.PicoInput8"))
  (:Triggered
    (Class|MetamorphopsiaController|UpdateScotoma (Variables|Default|GetmetaCon) (* (.y ActionValue) 0.1) (* (.x ActionValue) 0.1) (Variables|/Game/Blueprints/MetaCamera.MetaCamera_C|GetPlane (stale EventBeginPlay _asmeta_camera)))))

(event Input|EnhancedActionEvents|EnhancedInputActionPicoInputStore
  (params (ActionValue :type Boolean) (ElapsedSeconds :type Float%20%28double-precision%29) (TriggeredSeconds :type Float%20%28double-precision%29) (InputAction :type Input%20Action%20Object%20Reference :default "/Game/PicoInput/PicoInputStore.PicoInputStore"))
  (bind _metacon (Variables|Default|GetmetaCon))
  (Class|MetamorphopsiaController|SavePatientData _metacon (.layers (Variables|/Script/RAPD.MetamorphopsiaController|Getcurrent_scotoma _metacon)) false)
  (Game|OpenLevel(byName) "EyeTests"))

(event Input|EnhancedActionEvents|EnhancedInputActionPicoInputChangeEye
  (params (ActionValue :type Boolean) (ElapsedSeconds :type Float%20%28double-precision%29) (TriggeredSeconds :type Float%20%28double-precision%29) (InputAction :type Input%20Action%20Object%20Reference :default "/Game/PicoInput/PicoInputChangeEye.PicoInputChangeEye"))
  (bind _metacon (Variables|Default|GetmetaCon))
  (bind _rightui (Variables|Default|GetRightUI))
  (Utilities|FlowControl|FlipFlop
    (:A
      (Default|ChangeEye _rightui 1)
      (Class|MetamorphopsiaController|ChangeEye _metacon "Right" (Variables|/Game/Blueprints/MetaCamera.MetaCamera_C|GetPlane (stale EventBeginPlay _asmeta_camera))))
    (:B
      (Default|ChangeEye _rightui)
      (Class|MetamorphopsiaController|ChangeEye _metacon "Left" (Variables|/Game/Blueprints/MetaCamera.MetaCamera_C|GetPlane (stale EventBeginPlay _asmeta_camera))))))

(event Input|EnhancedActionEvents|EnhancedInputActionPicoInputEscape
  (params (ActionValue :type Boolean) (ElapsedSeconds :type Float%20%28double-precision%29) (TriggeredSeconds :type Float%20%28double-precision%29) (InputAction :type Input%20Action%20Object%20Reference :default "/Game/PicoInput/PicoInputEscape.PicoInputEscape"))
  (Utilities|FlowControl|FlipFlop
    (:A
      (Transformation|AddLocalOffset (Variables|/Game/Blueprints/MetaCamera.MetaCamera_C|GetPlane (stale EventBeginPlay _asmeta_camera)) "0.000000,0.000000,-160.000000" false false))
    (:B
      (Transformation|AddLocalOffset (Variables|/Game/Blueprints/MetaCamera.MetaCamera_C|GetPlane (stale EventBeginPlay _asmeta_camera)) "0.000000,0.000000,160.000000" false false))))

(event Input|EnhancedActionEvents|EnhancedInputActionPicoInputChangeProperty
  (params (ActionValue :type Boolean) (ElapsedSeconds :type Float%20%28double-precision%29) (TriggeredSeconds :type Float%20%28double-precision%29) (InputAction :type Input%20Action%20Object%20Reference :default "/Game/PicoInput/PicoInputChangeProperty.PicoInputChangeProperty"))
  ;[1 1 1] Change Property
  (Default|ChangeProperty (Variables|Default|GetLeftUI) true)
  (Class|MetamorphopsiaController|ChangeProperty (Variables|Default|GetmetaCon) true))

(event Input|EnhancedActionEvents|EnhancedInputActionPicoInputChangeLayer
  (params (ActionValue :type Boolean) (ElapsedSeconds :type Float%20%28double-precision%29) (TriggeredSeconds :type Float%20%28double-precision%29) (InputAction :type Input%20Action%20Object%20Reference :default "/Game/PicoInput/PicoInputChangeLayer.PicoInputChangeLayer"))
  (bind _metacon (Variables|Default|GetmetaCon))
  ;[1 1 1] Change Layer
  (bind _output_get (Variables|/Script/RAPD.MetamorphopsiaController|Setactive_layer _metacon (Math|Integer|%(Integer) (+ (Variables|/Script/RAPD.MetamorphopsiaController|Getactive_layer _metacon) 1) 3)))
  (Default|ChangeLayer (Variables|Default|GetLeftUI) _output_get))

(event EventBeginPlay
  (bind _returnvalue (Game|GetPlayerController 0))
  (bind _returnvalue_2 (PlayerController|LocalPlayerSubsystems|GetEnhancedInputLocalPlayerSubsystem _returnvalue))
  (bind _asmeta_camera (Utilities|Casting|CastToMetaCamera (Variables|/Script/Engine.ChildActorComponent|GetChildActor (Variables|Default|Getmeta_cam))))
  (bind _asmetamorphopsia_controller (Utilities|Casting|CastToMetamorphopsiaController (Variables|/Script/Engine.ChildActorComponent|GetChildActor (Variables|/Game/Blueprints/MetaCamera.MetaCamera_C|Getmeta_child _asmeta_camera))))
  (Variables|Default|SetmetaCon _asmetamorphopsia_controller)
  (Game|Player|SetViewTargetwithBlend (Game|GetPlayerController 0) _asmeta_camera 0.0 "VTBlend_Linear" 0.0 false)
  (bind _asui_meta_left (Utilities|Casting|CastToUI_Meta_Left (UserInterface|GetWidget (Variables|/Game/Blueprints/MetaCamera.MetaCamera_C|GetLeftUI _asmeta_camera))))
  (Variables|Default|SetLeftUI _asui_meta_left)
  (bind _asui_meta_right (Utilities|Casting|CastToUI_Meta_Right (UserInterface|GetWidget (Variables|/Game/Blueprints/MetaCamera.MetaCamera_C|GetRightUI _asmeta_camera))))
  (Variables|Default|SetRightUI _asui_meta_right)
  (Class|MetamorphopsiaController|GetStarted (Variables|Default|GetmetaCon) false (Variables|/Game/Blueprints/MetaCamera.MetaCamera_C|GetPlane _asmeta_camera) "/Game/Materials/Binocular/Binocular_Grid_Post.Binocular_Grid_Post" "/Game/Materials/Binocular/Binocular.Binocular")
  (Class|EnhancedInputSubsystemInterface|ClearAllMappings _returnvalue_2)
  (Input|AddMappingContext _returnvalue_2 "/Game/PicoInput/PicoEye.PicoEye" 100 "(bIgnoreAllPressedKeysUntilRelease=True,bForceImmediately=False,bNotifyUserSettings=False)"))

(event Input|KeyboardEvents|Add
  (params (Key :type Key%20Structure :default "None"))
  (:Pressed
    (Utilities|FlowControl|FlipFlop
      (:A
        (Transformation|AddLocalOffset (Variables|/Game/Blueprints/MetaCamera.MetaCamera_C|GetPlane (stale EventBeginPlay _asmeta_camera)) "0.000000,0.000000,-160.000000" false false))
      (:B
        (Transformation|AddLocalOffset (Variables|/Game/Blueprints/MetaCamera.MetaCamera_C|GetPlane (stale EventBeginPlay _asmeta_camera)) "0.000000,0.000000,160.000000" false false)))))

(event Input|KeyboardEvents|Subtract
  (params (Key :type Key%20Structure :default "None"))
  (:Pressed
    (Default|ChangeProperty (Variables|Default|GetLeftUI) true)
    (Class|MetamorphopsiaController|ChangeProperty (Variables|Default|GetmetaCon) true)))

(event Input|KeyboardEvents|Multiply
  (params (Key :type Key%20Structure :default "None"))
  (bind _metacon (Variables|Default|GetmetaCon))
  (:Pressed
    (bind _output_get (Variables|/Script/RAPD.MetamorphopsiaController|Setactive_layer _metacon (Math|Integer|%(Integer) (+ (Variables|/Script/RAPD.MetamorphopsiaController|Getactive_layer _metacon) 1) 3)))
    (Default|ChangeLayer (Variables|Default|GetLeftUI) _output_get)))

(event Input|KeyboardEvents|NumPadZero
  (params (Key :type Key%20Structure :default "None"))
  (bind _metacon (Variables|Default|GetmetaCon))
  (:Pressed
    (Class|MetamorphopsiaController|NewSimulation _metacon (Variables|/Game/Blueprints/MetaCamera.MetaCamera_C|GetPlane (stale EventBeginPlay _asmeta_camera)))
    (Default|Reset (Variables|Default|GetLeftUI))
    (Variables|/Script/RAPD.MetamorphopsiaController|Setselected_property _metacon 0)))

(fn ConstructionScript)