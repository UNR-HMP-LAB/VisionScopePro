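; TeleMedMode is a Blueprint, apparently the game mode for a telemedicine session, that runs a periodic check over the session's player states.
; Tick accumulates delta time and calls ShowName roughly once per second.
; ShowName casts each PlayerArray entry to PatientStatus and the game state to SessionStatus, but does nothing with the results, so no name is displayed.
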(event Custom|ShowName
  (bind _returnvalue (Game|GetGameState))
  (for _array_element (Variables|/Script/Engine.GameStateBase|GetPlayerArray _returnvalue)
    (Utilities|Casting|CastToPatientStatus _array_element))
  (Utilities|Casting|CastToSessionStatus _returnvalue))

(event EventBeginPlay)

(event EventTick
  (params (DeltaSeconds :type Float%20%28single-precision%29))
  (bind _output_get (Variables|Default|Setcurrent_time (+ (Variables|Default|Getcurrent_time) DeltaSeconds)))
  (if (> _output_get 1.0)
    (CallFunction|ShowName)
    (Variables|Default|Setcurrent_time 0.0)))

(fn ConstructionScript)