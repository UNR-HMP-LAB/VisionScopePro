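; PatientStatus is a player state for a patient session, tracking the player's identity and exposing session display data.
; On non-server instances, Tick copies name and type from the Visual_Function_Global game instance into Pid and debug-prints the type every frame.
; Getter functions read the SessionStatus game state for the current UI, post-process, meta changes, material, eye and scotoma.
; CopyProperties and TypePlayer are stubs that only cast or branch.
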(event EventBeginPlay)

(event EventCopyProperties
  (params (NewPlayerState :type Player%20State%20Object%20Reference))
  (Utilities|Casting|CastToPatientStatus NewPlayerState))

(event EventTick
  (params (DeltaSeconds :type Float%20%28single-precision%29))
  (if (not (Networking|IsServer))
    (bind _asvisual_function_global (Utilities|Casting|CastToVisual_Function_Global (Game|GetGameInstance)))
    (bind (_type _name) (Default|GetCurrentType _asvisual_function_global))
    (Variables|Default|Setpid (Utilities|Struct|MakePID _name "" _type))
    (Development|PrintString _type true true "(R=0.000000,G=0.660000,B=1.000000,A=1.000000)" 0.001)))

(fn ConstructionScript)

(fn TypePlayer
  (params (isDoctor :type Boolean))
  (Utilities|Casting|CastToVisual_Function_Global (Game|GetGameInstance))
  (if isDoctor
    _))

(fn PatientScreen
  (bind _assession_status (Utilities|Casting|CastToSessionStatus (Game|GetGameState)))
  (return (Variables|/Game/Blueprints/SessionStatus.SessionStatus_C|Getcurrent_ui _assession_status)))

(fn PatientMeta
  (bind _assession_status (Utilities|Casting|CastToSessionStatus (Game|GetGameState)))
  (return (Variables|/Game/Blueprints/SessionStatus.SessionStatus_C|Getpost_process _assession_status) (Variables|/Game/Blueprints/SessionStatus.SessionStatus_C|Getmeta_changes _assession_status) (Variables|/Game/Blueprints/SessionStatus.SessionStatus_C|Getmaterial _assession_status) (Variables|/Game/Blueprints/SessionStatus.SessionStatus_C|Geteye _assession_status) (Variables|/Game/Blueprints/SessionStatus.SessionStatus_C|Getcurrent_scotoma _assession_status)))