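; ColorCamera is a camera actor that presents a Trivector color-vision test, with its camera not locked to the HMD.
; On BeginPlay it tags the camera's child primitives with a custom depth stencil and gives the Canvas a dynamic material.
; TrivectorProtocol initializes color assist from device and plate CSVs, spawns stencil-tagged plates laid out relative to the camera view, passes them to CalLib, hides the Canvas and returns the stimulus direction and confusion line.
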(event EventBeginPlay
  (bind _cameracomponent (Variables|Default|GetCameraComponent))
  (Variables|/Script/Engine.CameraComponent|SetbLockToHmd _cameracomponent false)
  (for _array_element (Components|GetChildrenComponents _cameracomponent true)
    (bind _asprimitive_component (Utilities|Casting|CastToPrimitiveComponent _array_element))
    (Rendering|SetRenderCustomDepth _asprimitive_component true)
    (Rendering|SetCustomDepthStencilValue _asprimitive_component 5))
  (bind _returnvalue (Rendering|Material|CreateDynamicMaterialInstance "/Game/Canvas_material.Canvas_material" "None" "None" :!class /Script/Engine.KismetMaterialLibrary))
  (bind _output_get (Variables|Default|Setcanvas_mat _returnvalue))
  (Rendering|Material|SetMaterial (Variables|Default|GetCanvas) 0 _output_get))

(event Collision|EventActorBeginOverlap
  (params (OtherActor :type Actor%20Object%20Reference)))

(event EventTick
  (params (DeltaSeconds :type Float%20%28single-precision%29)))

(fn ConstructionScript)

(fn TrivectorProtocol
  (params (Device :type String))
  (bind _returnvalue (Utilities|String|Append Device ".csv"))
  (bind _cal_lib (Variables|Default|Getcal_lib))
  (bind _cameracomponent (Variables|Default|GetCameraComponent))
  (bind _all_plates (Variables|Default|Getall_plates))
  (Variables|/Script/RAPD.ColorCalibration|Setparent_mat (Variables|Default|Getcal_lib) "/Game/Canvas_material.Canvas_material")
  (Development|PrintString _returnvalue)
  (bind _all_plates_2 (Class|CalibratedCamera|InitializeColorAssist _returnvalue "points.csv" 0.09 48))
  (Utilities|Array|Clear (Variables|Default|Getall_plates))
  (for _array_element _all_plates_2
    (bind _output_get (Variables|Default|SetPlate_Transformation _array_element))
    ;[1 1 1] Spawns a Plate
    (bind _returnvalue_2 (Game|SpawnActorfromClass "/Game/plates.plates_C" (Math|Transform|MakeTransform (Math|Vector|MakeVector (.X (Math|Vector|BreakVector (+ (+ (+ (* (Math|Vector|GetForwardVector _cameracomponent) (Variables|Default|Getdistance)) (Transformation|GetWorldLocation _cameracomponent)) (* (Math|Vector|GetRightVector _cameracomponent) (.y (.Location (Math|Transform|BreakTransform _output_get))))) (* (Math|Vector|GetUpVector _cameracomponent) (.z (.Location (Math|Transform|BreakTransform _output_get))))))) (.Y (Math|Vector|BreakVector (+ (+ (+ (* (Math|Vector|GetForwardVector _cameracomponent) (Variables|Default|Getdistance)) (Transformation|GetWorldLocation _cameracomponent)) (* (Math|Vector|GetRightVector _cameracomponent) (.y (.Location (Math|Transform|BreakTransform _output_get))))) (* (Math|Vector|GetUpVector _cameracomponent) (.z (.Location (Math|Transform|BreakTransform _output_get))))))) (.Z (Math|Vector|BreakVector (+ (+ (+ (* (Math|Vector|GetForwardVector _cameracomponent) (Variables|Default|Getdistance)) (Transformation|GetWorldLocation _cameracomponent)) (* (Math|Vector|GetRightVector _cameracomponent) (.y (.Location (Math|Transform|BreakTransform _output_get))))) (* (Math|Vector|GetUpVector _cameracomponent) (.z (.Location (Math|Transform|BreakTransform _output_get)))))))) "0, 0, 0" (Math|Vector|MakeVector (/ (.y (.Scale (Math|Transform|BreakTransform _output_get))) 125.0) (/ (.y (.Scale (Math|Transform|BreakTransform _output_get))) 125.0) (/ (.y (.Scale (Math|Transform|BreakTransform _output_get))) 125.0))) "Undefined" "MultiplyWithRoot" 0 0))
    (Utilities|Array|Add _all_plates _returnvalue_2)
    (Rendering|SetRenderCustomDepth (Variables|/Script/Engine.StaticMeshActor|GetStaticMeshComponent _returnvalue_2) true)
    (Rendering|SetCustomDepthStencilValue (Variables|/Script/Engine.StaticMeshActor|GetStaticMeshComponent _returnvalue_2) 5))
  (Class|ColorCalibration|LoadAllPlatesMeshActor _cal_lib _all_plates)
  (bind (_confusion_line _direction) (Class|ColorCalibration|TrivectorTestStimuli _cal_lib))
  (Rendering|SetVisibility (Variables|Default|GetCanvas) false false)
  (return _direction _confusion_line))