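; Vision-test camera that presents Landolt C acuity (static or moving), Gabor contrast-sensitivity and reading stimuli, monocularly or binocularly.
; Acuity stimuli scale with camera distance to hold visual angle.
; Responses to randomized orientations drive adaptive logMAR sizing or step through log-spaced contrast levels until threshold.
; Per-eye post-process material instances apply metamorphopsia presets from the GameInstance and adjustable suppression; a toggle spawns and hides a handheld numpad.
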(event EventBeginPlay
  ;[1 1 1] log-linearly spaced contrast levels
  (Variables|Default|Settotal_CS_C 60)
  (for _index (range 0 (Variables|Default|Gettotal_CS_C))
    (Utilities|Array|Add (Variables|Default|Getmichelson_contrast_C) (Math|Float|Power 1e+01 (Math|Float|Lerp (Math|Float|Log 0.0015 1e+01) (Math|Float|Log 0.99 1e+01) (/ (Math|Conversions|ToFloat(Integer) _index) (Math|Conversions|ToFloat(Integer) (Variables|Default|Gettotal_CS_C)))))))
  (Class|EyeCamera|InitiatePostProcess))

(event Collision|EventActorBeginOverlap
  (params (OtherActor :type Actor%20Object%20Reference)))

(event EventTick
  (params (DeltaSeconds :type Float%20%28single-precision%29)))

(event EventSetOriginBound
  (params (origin :type Vector :default "0, 0, 0") (bound :type Float%20%28single-precision%29))
  ;[1 1 1] Set Boundary Origin
  (Variables|Default|Setpointer_origin_C origin)
  (Variables|Default|Setbound_C bound))

(event EventRandomOrientation
  (params (va :type Integer))
  ;[1 1 1] Set Orientations of Stimulus (8-directions)
  (bind _output_get (Variables|Default|Setprevious_orientation_C (Variables|Default|Getcurrent_orientation_C)))
  (bind _output_get_2 (Variables|Default|Setcurrent_orientation_C (Math|Integer|%(Integer) (+ _output_get (* (Math|Random|RandomIntegerinRange 1 3) 2)) (Utilities|Array|Get(acopy) (Utilities|Array|MakeArray 4 8) va))))
  (Rendering|Material|SetScalarParameterValue (Variables|Default|Getcurrent_optotype_C) "orientation" (Utilities|Array|Get(acopy) (Utilities|Array|MakeArray 0.0 0.125 0.25 0.375 0.5 0.625 0.75 0.875) _output_get_2) :!class /Script/Engine.MaterialInstanceDynamic))

(event EventMoveAlong
  (params (times :type Float%20%28single-precision%29) (dir :type Vector :default "0, 0, 0"))
  ;[1 1 1] Move the Stimulus Along and Away
  (Transformation|AddWorldOffset (Variables|Default|GetPlane) (* (Math|Vector|Normalize dir) times) true false))

(event EventMonocularLeft
  (bind _plane (Variables|Default|GetPlane))
  (bind _plane1 (Variables|Default|GetPlane1))
  ;[1 1 1] Set Left Material Instance
  (bind _returnvalue (Rendering|Material|CreateDynamicMaterialInstance _plane 0 "/Game/Materials/Landolt_C_Left.Landolt_C_Left" "None" :!class /Script/Engine.PrimitiveComponent))
  (Variables|Default|Setcurrent_optotype_C _returnvalue)
  (Variables|Default|Setwhich_eye_C "Left")
  (Rendering|Material|SetMaterial _plane1 0 "/Game/Materials/light_l.light_l") ; If want screen black use light_l
  ;[1 1 1] Present Stimjlus at Correct Scale
  (bind _distance (CallFunction|GetDistance))
  (Transformation|SetRelativeScale3D _plane (Math|Vector|MakeVector (* _distance (Math|Trig|Tan(Degrees) (/ 2e+01 12.0))) (* _distance (Math|Trig|Tan(Degrees) (/ 2e+01 12.0))) 0.1))
  (Variables|Default|Settotal_seen_C 0)
  (Rendering|SetVisibility _plane1 true false)
  (Variables|Default|Setcurrent_log_C 1.3)
  (Variables|Default|Setprevious_log_C 1.4))

(event EventMonocularRight
  (bind _plane (Variables|Default|GetPlane))
  (bind _plane1 (Variables|Default|GetPlane1))
  ;[1 1 1] Set Right Material
  (bind _returnvalue (Rendering|Material|CreateDynamicMaterialInstance _plane 0 "/Game/Materials/Landolt_C_Right.Landolt_C_Right" "None" :!class /Script/Engine.PrimitiveComponent))
  (Variables|Default|Setcurrent_optotype_C _returnvalue)
  (Variables|Default|Setwhich_eye_C "Right")
  (Rendering|Material|SetMaterial _plane1 0 "/Game/Materials/light_r.light_r") ; If want screen black use light_r
  ;[1 1 1] Present Stimjlus at Correct Scale
  (bind _distance (CallFunction|GetDistance))
  (Transformation|SetRelativeScale3D _plane (Math|Vector|MakeVector (* _distance (Math|Trig|Tan(Degrees) (/ 2e+01 12.0))) (* _distance (Math|Trig|Tan(Degrees) (/ 2e+01 12.0))) 0.1))
  (Variables|Default|Settotal_seen_C 0)
  (Rendering|SetVisibility _plane1 true false)
  (Variables|Default|Setcurrent_log_C 1.3)
  (Variables|Default|Setprevious_log_C 1.4))

(event EventBinocularStatic
  (bind _plane (Variables|Default|GetPlane))
  (bind _plane1 (Variables|Default|GetPlane1))
  ;[1 1 1] Create Materials for Visual Acutiy for Both Eyes
  (Variables|Default|Setwhich_eye_C "Binocular")
  (bind _returnvalue (Rendering|Material|CreateDynamicMaterialInstance _plane 0 "/Game/Materials/Landolt_C.Landolt_C" "None" :!class /Script/Engine.PrimitiveComponent))
  (Variables|Default|Setcurrent_optotype_C _returnvalue)
  (Rendering|Material|SetMaterial _plane1 0 "/Game/Materials/light.light")
  ;[1 1 1] Present Stimjlus at Correct Scale
  (bind _distance (CallFunction|GetDistance))
  (Transformation|SetRelativeScale3D _plane (Math|Vector|MakeVector (* _distance (Math|Trig|Tan(Degrees) (/ 2e+01 12.0))) (* _distance (Math|Trig|Tan(Degrees) (/ 2e+01 12.0))) 0.1))
  (Variables|Default|Settotal_seen_C 0)
  (Rendering|SetVisibility _plane1 true false)
  (Variables|Default|Setcurrent_log_C 1.3)
  (Variables|Default|Setprevious_log_C 1.4))

(event EventBinocularDynamic
  (bind _plane (Variables|Default|GetPlane))
  (bind _plane1 (Variables|Default|GetPlane1))
  ;[1 1 1] Create Materials for Visual Acutiy for Both Eyes
  (Variables|Default|Setwhich_eye_C "Dynamic")
  (Class|EyeCamera|SetOriginBound "299.000000,0.000000,0.000000" 5e+01)
  (bind _returnvalue (Rendering|Material|CreateDynamicMaterialInstance _plane 0 "/Game/Materials/Landolt_C.Landolt_C" "None" :!class /Script/Engine.PrimitiveComponent))
  (Variables|Default|Setcurrent_optotype_C _returnvalue)
  (Rendering|Material|SetMaterial _plane1 0 "/Game/Materials/light.light")
  ;[1 1 1] Present Stimjlus at Correct Scale
  (bind _distance (CallFunction|GetDistance))
  (Transformation|SetRelativeScale3D _plane (Math|Vector|MakeVector (* _distance (Math|Trig|Tan(Degrees) (/ 2e+01 12.0))) (* _distance (Math|Trig|Tan(Degrees) (/ 2e+01 12.0))) 0.1))
  (Variables|Default|Settotal_seen_C 0)
  (Rendering|SetVisibility _plane1 true false)
  (Variables|Default|Setcurrent_log_C 1.3)
  (Variables|Default|Setprevious_log_C 1.4))

(event EventCS
  (bind _plane1 (Variables|Default|GetPlane1))
  (bind _plane (Variables|Default|GetPlane))
  ;[1 1 1] Create Materials for Contrast Sensitivity for Each Eye
  (Variables|Default|Setwhich_eye_C "Left")
  (bind _returnvalue (Rendering|Material|CreateDynamicMaterialInstance _plane 0 "/Game/Materials/gabor_patches.gabor_patches" "None" :!class /Script/Engine.PrimitiveComponent))
  (bind _output_get (Variables|Default|Setcurrent_optotype_C _returnvalue))
  (Rendering|Material|SetScalarParameterValue _output_get "monocular_r" 0.0 :!class /Script/Engine.MaterialInstanceDynamic)
  (bind _distance (CallFunction|GetDistance))
  (Transformation|SetRelativeScale3D _plane (Math|Vector|MakeVector (* _distance (Math|Trig|Tan(Degrees) 12.0)) (* _distance (Math|Trig|Tan(Degrees) 12.0)) 0.1))
  (Variables|Default|Settotal_seen_C 46)
  (Variables|Default|Setcount_right_C 5)
  (Rendering|SetVisibility _plane1 true false)
  (Rendering|Material|SetMaterial _plane1 0 "/Game/Materials/background.background")
  (Variables|Default|Setcurrent_log_C 1.3)
  (Variables|Default|Setprevious_log_C 1.4))

(event EventCSRight
  (bind _plane1 (Variables|Default|GetPlane1))
  (bind _plane (Variables|Default|GetPlane))
  ;[1 1 1] Create Materials for Contrast Sensitivity for Each Eye
  (Variables|Default|Setwhich_eye_C "Right")
  (bind _returnvalue (Rendering|Material|CreateDynamicMaterialInstance _plane 0 "/Game/Materials/gabor_patches.gabor_patches" "None" :!class /Script/Engine.PrimitiveComponent))
  (bind _output_get (Variables|Default|Setcurrent_optotype_C _returnvalue))
  (Rendering|Material|SetScalarParameterValue _output_get "monocular_l" 0.0 :!class /Script/Engine.MaterialInstanceDynamic)
  (bind _distance (CallFunction|GetDistance))
  (Transformation|SetRelativeScale3D _plane (Math|Vector|MakeVector (* _distance (Math|Trig|Tan(Degrees) 12.0)) (* _distance (Math|Trig|Tan(Degrees) 12.0)) 0.1))
  (Variables|Default|Settotal_seen_C 46)
  (Variables|Default|Setcount_right_C 5)
  (Rendering|SetVisibility _plane1 true false)
  (Rendering|Material|SetMaterial _plane1 0 "/Game/Materials/background.background")
  (Variables|Default|Setcurrent_log_C 1.3)
  (Variables|Default|Setprevious_log_C 1.4))

(event EventInitiatePostProcess
  ;[1 1 1] Post Processing
  (bind _returnvalue (Rendering|Material|CreateDynamicMaterialInstance "/Game/Materials/Binocular/Binocular_Grid_Post.Binocular_Grid_Post" "Left" "None" :!class /Script/Engine.KismetMaterialLibrary))
  (Variables|Default|Setleft_C _returnvalue)
  (bind _returnvalue_2 (Rendering|Material|CreateDynamicMaterialInstance "/Game/Materials/Binocular/testing_R.testing_R" "Right" "None" :!class /Script/Engine.KismetMaterialLibrary))
  (Variables|Default|Setright_C _returnvalue_2)
  (Class|EyeCamera|SetMaterialtoPost))

(event EventReadingTest
  (bind _plane (Variables|Default|GetPlane))
  (bind _plane1 (Variables|Default|GetPlane1))
  ;[1 1 1] Create Materials for the Reading Test
  (Variables|Default|Setscale 3.0)
  (Rendering|Material|CreateDynamicMaterialInstance _plane 0 "/Game/Materials/Lorem/lorem_ipsum_Inst.lorem_ipsum_Inst" "None" :!class /Script/Engine.PrimitiveComponent)
  (Transformation|SetRelativeScale3D _plane (Math|Vector|MakeVector (Variables|Default|Getscale) (Variables|Default|Getscale) 0.1))
  (Rendering|SetVisibility _plane1 true false)
  (Rendering|Material|SetMaterial _plane1 0 "/Game/Materials/light.light"))

(event EventSetMaterialtoPost
  (bind _post_process_c (Variables|Default|Getpost_process_C))
  (bind _right_c (Variables|Default|Getright_C))
  ;[1 1 1] Set Material to Postprocess (?)
  (Utilities|Array|Clear _post_process_c)
  (Utilities|Array|Add _post_process_c (Utilities|Struct|MakePostProcessSettings (Utilities|Struct|MakeWeightedBlendables (Utilities|Array|MakeArray (Utilities|Struct|MakeWeightedBlendable 1.0 (Variables|Default|Getleft_C))))))
  (Utilities|Array|Add _post_process_c (Utilities|Struct|MakePostProcessSettings (Utilities|Struct|MakeWeightedBlendables (Utilities|Array|MakeArray (Utilities|Struct|MakeWeightedBlendable 1.0 _right_c)))))
  (Rendering|Material|GetScalarParameterValue _right_c "Right_Rotation0" :!class /Script/Engine.MaterialInstanceDynamic))

(event EventDifferentSuppression
  (params (up :type Boolean))
  ;[1 1 1] Different Suppression
  (if up
    (bind _result (Math|Integer|IncrementInt (Variables|Default|Getcurrent_suppression_C))
      (:%20%20
        (if (== _result 4)
          (Variables|Default|Setcurrent_suppression_C 0))))
    (else
      (bind _result_2 (Math|Integer|DecrementInt (Variables|Default|Getcurrent_suppression_C))
        (:%20%20
          (if (== _result_2 -1)
            (Variables|Default|Setcurrent_suppression_C 3))))))
  (bind _name (CallFunction|ApplyBino "Sigma1"))
  (bind _name_2 (CallFunction|ApplyBino "Weight1"))
  (bind _name_3 (CallFunction|ApplyBino "Sigma0"))
  (switch string (Variables|Default|Getwhich_eye_C)
    (:Left
      (Variables|Default|Setdistortion (Variables|Default|Getleft_C)))
    (:Right
      (Variables|Default|Setdistortion (Variables|Default|Getright_C))))
  (bind _returnvalue (Rendering|Material|GetScalarParameterValue (Variables|Default|Getdistortion) _name_3 :!class /Script/Engine.MaterialInstanceDynamic))
  (switch int (Variables|Default|Getcurrent_suppression_C)
    (:0
      (Rendering|Material|SetScalarParameterValue (Variables|Default|Getdistortion) _name 0.0 :!class /Script/Engine.MaterialInstanceDynamic))
    (:1
      (Rendering|Material|SetScalarParameterValue (Variables|Default|Getdistortion) _name (/ _returnvalue 5.0) :!class /Script/Engine.MaterialInstanceDynamic))
    (:2
      (Rendering|Material|SetScalarParameterValue (Variables|Default|Getdistortion) _name (/ _returnvalue 1.8) :!class /Script/Engine.MaterialInstanceDynamic))
    (:3
      (Rendering|Material|SetScalarParameterValue (Variables|Default|Getdistortion) _name (/ _returnvalue 1.2) :!class /Script/Engine.MaterialInstanceDynamic)))
  (Rendering|Material|SetScalarParameterValue (Variables|Default|Getdistortion) _name_2 1.0 :!class /Script/Engine.MaterialInstanceDynamic))

(fn ConstructionScript)

(fn MovePointer
  (params (direction :type Vector :default "0, 0, 0") (speed :type Float%20%28single-precision%29))
  (bind _plane (Variables|Default|GetPlane))
  (bind _returnvalue (Transformation|GetWorldLocation _plane))
  ;[1 1 1] Within Bound?
  (if (< (Variables|Default|Getbound_C) (Math|Vector|Distance(Vector) (Variables|Default|Getpointer_origin_C) _returnvalue))
    ;[1 1 1] Go Towards Origin
    (bind _new_direction (CallFunction|TowardsOrigin _returnvalue))
    (Class|EyeCamera|MoveAlong speed _new_direction)
    (return _new_direction)
    (else
      ;[1 1 1] Go Forward
      (Class|EyeCamera|MoveAlong speed direction)
      (return direction))))

(fn TowardsOrigin
  (params (location :type Vector :default "0, 0, 0"))
  (return (- (Variables|Default|Getpointer_origin_C) location)))

(fn ResizeOptotype
  (if (> (Variables|Default|Getcount_right_C) 2)
    (Variables|Default|Setprevious_log_C (Variables|Default|Getcurrent_log_C))
    (Variables|Default|Setcurrent_log_C (- (Variables|Default|Getcurrent_log_C) 0.1))
    (else
      (Variables|Default|Setcurrent_log_C (/ (+ (Variables|Default|Getprevious_log_C) (Variables|Default|Getcurrent_log_C)) 2.0))))
  ;[1 1 1] Reached threshold
  (if (< (Math|Float|Absolute(Float) (- (Variables|Default|Getcurrent_log_C) (Variables|Default|Getprevious_log_C))) 0.03)
    (Variables|Default|Setcount_right_C 0)
    (return true)
    (else
      ;[1 1 1] New Gap Size
      (bind _output_get (Variables|Default|Setgap_C (Math|Float|Power 1e+01 (Variables|Default|Getcurrent_log_C))))
      (bind _distance (CallFunction|GetDistance))
      (Transformation|SetWorldScale3D (Variables|Default|GetPlane) (Math|Vector|MakeVector (* (Math|Trig|Tan(Degrees) (/ _output_get 12.0)) _distance) (* (Math|Trig|Tan(Degrees) (/ _output_get 12.0)) _distance) 0.1))
      (Class|EyeCamera|RandomOrientation 1)
      (Variables|Default|Setcount_right_C 0)
      (return false))))

(fn AssessResponses
  (params (ro :type String) (test :type String))
  (bind _current_optotype_c (Variables|Default|Getcurrent_optotype_C))
  (if (== (Utilities|Array|Get(acopy) (Utilities|Array|MakeArray 0.0 0.125 0.25 0.375 0.5 0.625 0.75 0.875) (Variables|Default|Getcurrent_orientation_C)) (.Value (Utilities|Map|Find (Variables|Default|Getmapping_C) ro)))
    (Variables|Default|Setrecent_right_C true)
    (switch string test
      (:Reading%20Test
        (Variables|Default|Setscale (/ (Variables|Default|Getscale) 1.25)))
      (:Static%20VA%20Bino
        (bind _result (Math|Integer|IncrementInt (Variables|Default|Getcount_right_C) :!label _label)
          (:%20%20
            (if (> _result 2)
              _
              (else
                (bind _result_2 (Math|Integer|IncrementInt (Variables|Default|Gettotal_seen_C) :!label _label_2)
                  (:%20%20
                    (if (== _result_2 5)
                      _
                      (else
                        (Class|EyeCamera|RandomOrientation 1)
                        (return false)))))))
            (Variables|Default|Settotal_seen_C 0)
            (bind _completed (CallFunction|ResizeOptotype))
            (return _completed))))
      (:Static%20VA%20Mono
        (goto _label))
      (:Dynamic%20VA
        (goto _label))
      (:CS%20Mono
        (Rendering|Material|SetScalarParameterValue _current_optotype_c "contrast ratio" (Utilities|Array|Get(acopy) (Variables|Default|Getmichelson_contrast_C) (Variables|Default|Gettotal_seen_C)) :!class /Script/Engine.MaterialInstanceDynamic)
        (bind _result_3 (Math|Integer|DecrementInt (Variables|Default|Gettotal_seen_C))
          (:%20%20
            (if (> 0 _result_3)
              (return true)
              (else
                (Class|EyeCamera|RandomOrientation)
                (return false)))))))
    (else
      (Variables|Default|Setrecent_right_C false)
      (switch string test
        (:Reading%20Test
          (Variables|Default|Setscale (* (Variables|Default|Getscale) 1.25)))
        (:Static%20VA%20Bino
          (goto _label_2))
        (:Static%20VA%20Mono
          (goto _label_2))
        (:Dynamic%20VA
          (goto _label_2))
        (:CS%20Mono
          (Rendering|Material|SetScalarParameterValue _current_optotype_c "contrast ratio" (Utilities|Array|Get(acopy) (Variables|Default|Getmichelson_contrast_C) (Variables|Default|Gettotal_seen_C)) :!class /Script/Engine.MaterialInstanceDynamic)
          (bind _result_4 (Math|Integer|DecrementInt (Variables|Default|Getcount_right_C))
            (:%20%20
              (if (< _result_4 3)
                (return true)
                (else
                  (Class|EyeCamera|RandomOrientation)
                  (return false)))))))))
  (Transformation|SetWorldScale3D (Variables|Default|GetPlane) (Math|Vector|MakeVector (Variables|Default|Getscale) (Variables|Default|Getscale) 0.1)))

(fn GetDistance
  (return (/ (Math|Vector|Distance(Vector) (Transformation|GetWorldLocation (Variables|Default|GetPlane)) (Transformation|GetWorldLocation (Variables|Default|GetCameraComponent))) 1e+02)))

(fn LoadMetamorphopsia
  (params (up :type Boolean))
  (bind _left_c (Variables|Default|Getleft_C))
  (bind _right_c (Variables|Default|Getright_C))
  ;[1 1 1] Gaze Update
  (bind _asvisual_function_global (Utilities|Casting|CastToVisual_Function_Global (Game|GetGameInstance)))
  (Default|InitializeScotoma _asvisual_function_global)
  (if up
    (Variables|Default|Setcurrent_metamorphopsia_C (Math|Integer|%(Integer) (+ (Variables|Default|Getcurrent_metamorphopsia_C) 1) 6))
    (else
      (bind _output_get (Variables|Default|Setcurrent_metamorphopsia_C (Math|Integer|%(Integer) (+ (Variables|Default|Getcurrent_metamorphopsia_C) 5) 6)))))
  (bind _name (CallFunction|ApplyBino "Mean0"))
  (bind _name_2 (CallFunction|ApplyBino "Mean1"))
  (switch string (Variables|Default|Getwhich_eye_C)
    (:Left
      (Rendering|Material|SetVectorParameterValue _left_c _name (.meancolor (Utilities|Array|Get(acopy) (Variables|/Game/Blueprints/Visual_Function_Global.Visual_Function_Global_C|Gettemp_meta _asvisual_function_global) (Variables|Default|Getcurrent_metamorphopsia_C))) :!class /Script/Engine.MaterialInstanceDynamic)
      (Rendering|Material|SetVectorParameterValue _left_c _name_2 (.meancolor (Utilities|Array|Get(acopy) (Variables|/Game/Blueprints/Visual_Function_Global.Visual_Function_Global_C|Gettemp_meta _asvisual_function_global) (Variables|Default|Getcurrent_metamorphopsia_C))) :!class /Script/Engine.MaterialInstanceDynamic))
    (:Right
      (Rendering|Material|SetVectorParameterValue _right_c _name (Math|Color|MakeColor (- (.R (Math|Color|BreakColor (.meancolor (Utilities|Array|Get(acopy) (Variables|/Game/Blueprints/Visual_Function_Global.Visual_Function_Global_C|Gettemp_meta _asvisual_function_global) (Variables|Default|Getcurrent_metamorphopsia_C))))) 0.062) (+ (.G (Math|Color|BreakColor (.meancolor (Utilities|Array|Get(acopy) (Variables|/Game/Blueprints/Visual_Function_Global.Visual_Function_Global_C|Gettemp_meta _asvisual_function_global) (Variables|Default|Getcurrent_metamorphopsia_C))))) 0.005) 0.0 (.A (Math|Color|BreakColor (.meancolor (Utilities|Array|Get(acopy) (Variables|/Game/Blueprints/Visual_Function_Global.Visual_Function_Global_C|Gettemp_meta _asvisual_function_global) (Variables|Default|Getcurrent_metamorphopsia_C)))))) :!class /Script/Engine.MaterialInstanceDynamic)
      (Rendering|Material|SetVectorParameterValue _right_c _name_2 (Math|Color|MakeColor (- (.R (Math|Color|BreakColor (.meancolor (Utilities|Array|Get(acopy) (Variables|/Game/Blueprints/Visual_Function_Global.Visual_Function_Global_C|Gettemp_meta _asvisual_function_global) (Variables|Default|Getcurrent_metamorphopsia_C))))) 0.062) (+ (.G (Math|Color|BreakColor (.meancolor (Utilities|Array|Get(acopy) (Variables|/Game/Blueprints/Visual_Function_Global.Visual_Function_Global_C|Gettemp_meta _asvisual_function_global) (Variables|Default|Getcurrent_metamorphopsia_C))))) 0.005) 0.0 (.A (Math|Color|BreakColor (.meancolor (Utilities|Array|Get(acopy) (Variables|/Game/Blueprints/Visual_Function_Global.Visual_Function_Global_C|Gettemp_meta _asvisual_function_global) (Variables|Default|Getcurrent_metamorphopsia_C)))))) :!class /Script/Engine.MaterialInstanceDynamic)))
  (for (_array_element _array_index) (Utilities|Array|MakeArray (.sigma (Utilities|Array|Get(acopy) (Variables|/Game/Blueprints/Visual_Function_Global.Visual_Function_Global_C|Gettemp_meta _asvisual_function_global) (Variables|Default|Getcurrent_metamorphopsia_C))) (.weight (Utilities|Array|Get(acopy) (Variables|/Game/Blueprints/Visual_Function_Global.Visual_Function_Global_C|Gettemp_meta _asvisual_function_global) (Variables|Default|Getcurrent_metamorphopsia_C))) (.rotation (Utilities|Array|Get(acopy) (Variables|/Game/Blueprints/Visual_Function_Global.Visual_Function_Global_C|Gettemp_meta _asvisual_function_global) (Variables|Default|Getcurrent_metamorphopsia_C))) (.distortion (Utilities|Array|Get(acopy) (Variables|/Game/Blueprints/Visual_Function_Global.Visual_Function_Global_C|Gettemp_meta _asvisual_function_global) (Variables|Default|Getcurrent_metamorphopsia_C))))
    (switch string (Variables|Default|Getwhich_eye_C)
      (:Left
        (bind _name_3 (CallFunction|ApplyBino (Utilities|String|Append (Utilities|Array|Get(acopy) (Variables|Default|Getscotoma_parameters_C) _array_index) "0")))
        (Rendering|Material|SetScalarParameterValue _left_c _name_3 _array_element :!class /Script/Engine.MaterialInstanceDynamic))
      (:Right
        (bind _name_4 (CallFunction|ApplyBino (Utilities|String|Append (Utilities|Array|Get(acopy) (Variables|Default|Getscotoma_parameters_C) _array_index) "0")))
        (Rendering|Material|SetScalarParameterValue _right_c _name_4 _array_element :!class /Script/Engine.MaterialInstanceDynamic)))
    (return _output_get)))

(fn ObtainResults
  (params (test :type String))
  (switch string test
    (:Static%20VA%20Bino
      _)
    (:Static%20VA%20Mono
      _)
    (:Dynamic%20VA
      _)
    (:CS%20Mono
      (bind _logcs (CallFunction|FromMichelson (Utilities|Array|Get(acopy) (Variables|Default|Getmichelson_contrast_C) (Variables|Default|Gettotal_seen_C))))
      (return _logcs)))
  (bind _output_get (Variables|Default|Setgap_C (Math|Float|Power 1e+01 (Variables|Default|Getcurrent_log_C))))
  (bind _logmar (CallFunction|FromGap _output_get))
  (return _logmar))

(fn ApplyBino
  (params (test :type String))
  (return (Utilities|String|StringToName (Utilities|String|Append (Variables|Default|Getwhich_eye_C) "_" test))))

(fn ToggleNumpad
  (Variables|Default|GetnumpadRef
    (:then
      (Utilities|FlowControl|FlipFlop
        (:A
          (Transformation|SetRelativeScale3D (Variables|/Game/handheld.handheld_C|GetWidget (stale _output_get)) "0, 0, 0"))
        (:B
          (Transformation|SetRelativeScale3D (Variables|/Game/handheld.handheld_C|GetWidget (stale _output_get)) (Math|Conversions|ToVector(Float) (Variables|Default|GetWidgetRelativeScaleOriginal))))))
    (:else
      (bind _returnvalue (Game|SpawnActorfromClass "/Game/handheld.handheld_C" (Math|Transform|MakeTransform "0, 0, 0" "0, 0, 0" "1.000000,1.000000,1.000000") "Undefined" "OverrideRootScale" 0 0))
      (bind _output_get (Variables|Default|SetnumpadRef _returnvalue))
      (Variables|Default|SetWidgetRelativeScaleOriginal (.x (Variables|/Script/Engine.SceneComponent|GetRelativeScale3D (Variables|/Game/handheld.handheld_C|GetWidget _output_get)))) ; Set the original relative scale
    )))