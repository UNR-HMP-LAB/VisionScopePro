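; SessionStatus is a game-state Blueprint that tracks patients in a multiplayer session, apparently for visual function work.
; On server Tick, while player count differs from Stored, it scans PatientStatus entries, registers "copied" PIDs and copies non-zero gaze vectors.
; UpdatePID appends IDs not found in its lists, and Tick also mirrors the game instance's CurrentPatient into SelectedPatient.
; UpdateButtons increments per-player timers but is not called here.
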(event EventBeginPlay
  (Variables|Default|Settimes (Utilities|Array|MakeArray 0.0 0.0 0.0)))

(event EventTick
  (params (DeltaSeconds :type Float%20%28single-precision%29))
  (bind _playerarray (Variables|Default|GetPlayerArray))
  (bind _returnvalue (Utilities|Array|Length _playerarray))
  (if (Networking|IsServer)
    (Utilities|FlowControl|Sequence
      (:then_0
        (if (not (== _returnvalue (Variables|Default|Getstored)))
          (for _index (range 1 _returnvalue)
            (bind _aspatient_status (Utilities|Casting|CastToPatientStatus (Utilities|Array|Get(acopy) _playerarray _index)))
            (Utilities|FlowControl|Sequence
              (:then_0
                (if (Utilities|Enum|Equal(Enum) (.type (Variables|/Game/Blueprints/PatientStatus.PatientStatus_C|Getpid _aspatient_status)) "copied")
                  (Variables|Default|Setstored _returnvalue)
                  (CallFunction|UpdatePID (Utilities|Struct|MakePID (PlayerState|GetPlayerName _aspatient_status) (.pass (Variables|/Game/Blueprints/PatientStatus.PatientStatus_C|Getpid _aspatient_status)) "Patient"))))
              (:then_1
                (if (not (Math|Vector|Equal(Vector) (Variables|/Game/Blueprints/PatientStatus.PatientStatus_C|Getgaze_vector _aspatient_status) "0, 0, 0" 0.0001))
                  (Variables|Default|Setgaze_vector (Variables|/Game/Blueprints/PatientStatus.PatientStatus_C|Getgaze_vector _aspatient_status))))))))
      (:then_1
        (bind _asvisual_function_global (Utilities|Casting|CastToVisual_Function_Global (Game|GetGameInstance)))
        (Variables|Default|Setselected_patient (Variables|/Game/Blueprints/Visual_Function_Global.Visual_Function_Global_C|Getcurrent_patient _asvisual_function_global))))))

(fn ConstructionScript)

(fn UpdateButtons
  (bind _playerarray (Variables|Default|GetPlayerArray))
  (bind _times (Variables|Default|Gettimes))
  (bind _returnvalue (Utilities|Array|Length _playerarray))
  (if (> _returnvalue 1)
    (for _index (range 0 (- _returnvalue 2))
      (Utilities|Array|SetArrayElem _times _index (+ (Utilities|Array|Get(acopy) _times _index) 0.01)))))

(fn UpdatePID
  (params (PID :type PID%20Structure))
  (bind _ids (Variables|Default|Getids))
  (Development|PrintString (.id PID) true true "(R=0.000000,G=0.660000,B=1.000000,A=1.000000)" 1e+01)
  (for _array_element _ids
    (if (LocalVariables|GetNot%20found)
      (bind _output_get (LocalVariables|SetNot%20found (Utilities|Enum|NotEqual(Enum) _array_element (.id PID))))
      (if _output_get
        _)))
  (if (LocalVariables|GetNot%20found)
    (Utilities|Array|Add _ids (.id PID))
    (Utilities|Array|Add (Variables|Default|Getpids) (Utilities|Struct|MakePID (.id PID) (.pass PID) (.type PID)))))