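; BP_NASA_Pawn is a VR pawn that sets up Pico controller laser input and a test menu widget.
; On BeginPlay it adds the PicoNASA Enhanced Input mapping, sets floor tracking origin and registers its NASATestMenu widget as StartUI on the game instance.
; The Pico click action presses and releases the left mouse pointer key on both controller lasers at once, with debug prints.
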(event Input|EnhancedActionEvents|EnhancedInputActionPicoInputOnClick
  (params (ActionValue :type Boolean) (ElapsedSeconds :type Float%20%28double-precision%29) (TriggeredSeconds :type Float%20%28double-precision%29) (InputAction :type Input%20Action%20Object%20Reference :default "/Game/PicoInput/PicoInputOnClick.PicoInputOnClick"))
  (:Started
    (Class|WidgetInteractionComponent|PressPointerKey (Variables|Default|GetControllerLaser_Right) "LeftMouseButton")
    (Development|PrintString "Pressed."))
  (:Completed
    (Class|WidgetInteractionComponent|ReleasePointerKey (Variables|Default|GetControllerLaser_Left) "LeftMouseButton")
    (Development|PrintString "Released.")))

(event EventBeginPlay
  (Input|AddMappingContext (PlayerController|LocalPlayerSubsystems|GetEnhancedInputLocalPlayerSubsystem (Game|GetPlayerController 0)) "/Game/PicoInput/PicoNASA.PicoNASA" 10 "(bIgnoreAllPressedKeysUntilRelease=True,bForceImmediately=False,bNotifyUserSettings=False)")
  (Development|PrintString "Using Enhanced Inputs." true true "(R=0.000000,G=0.660000,B=1.000000,A=1.000000)" 15.0)
  (Class|HeadMountedDisplayFunctionLibrary|SetTrackingOrigin "Floor")
  (bind _asbp_nasagame_instance (Utilities|Casting|CastToBP_NASAGameInstance (Game|GetGameInstance)))
  (bind _asbp_nasatest_menu (Utilities|Casting|CastToBP_NASATestMenu (UserInterface|GetUserWidgetObject (Variables|Default|GetNASATestMenu))))
  (Variables|/Game/Blueprints/BP_NASAGameInstance.BP_NASAGameInstance_C|SetStartUI _asbp_nasagame_instance _asbp_nasatest_menu))

(event EventTick
  (params (DeltaSeconds :type Float%20%28single-precision%29)))

(fn ConstructionScript)