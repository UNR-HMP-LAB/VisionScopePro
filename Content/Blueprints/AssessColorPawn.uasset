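; Pawn that runs a trivector color vision assessment on Pico input, viewed through a child ColorCamera.
; BeginPlay loads or creates the patient save and fills the menu; Enter or Space swaps menu for canvas and starts the protocol.
; Directional responses feed CalLib, restart a timed obscuring sphere, and finally record CSV, save and open ColorTest.
; Post-protocol setup, including setting the Done flag that gates responses, is unwired.
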(event Custom|count_start
  (Utilities|Time|SetTimerbyEvent (delegate Custom|obscure) 3.0))

(event Custom|obscure
  (Rendering|SetVisibility (Variables|/Game/Blueprints/ColorCamera.ColorCamera_C|GetSphere (Variables|Default|GetthisColorCamera)) true false)
  (Development|PrintString "Timer hit."))

(event Custom|unobscure
  (Rendering|SetVisibility (Variables|/Game/Blueprints/ColorCamera.ColorCamera_C|GetSphere (Variables|Default|GetthisColorCamera)) false false))

(event Input|EnhancedActionEvents|EnhancedInputActionPicoInputEnter
  (params (ActionValue :type Boolean) (ElapsedSeconds :type Float%20%28double-precision%29) (TriggeredSeconds :type Float%20%28double-precision%29) (InputAction :type Input%20Action%20Object%20Reference :default "/Game/PicoInput/PicoInputEnter.PicoInputEnter"))
  (bind _thiscolorcamera (Variables|Default|GetthisColorCamera))
  (Development|PrintString "Pico Triggered")
  (Utilities|FlowControl|DoOnce false
    (:Completed
      (Rendering|SetVisibility (Variables|/Game/Blueprints/ColorCamera.ColorCamera_C|Getui _thiscolorcamera) false true)
      (Rendering|SetVisibility (Variables|/Game/Blueprints/ColorCamera.ColorCamera_C|GetCanvas _thiscolorcamera) true true)
      ;[1 1 1] Connect These two
      (bind _device (Default|Selections (Variables|Default|Getui)))
      (bind _output_get (Variables|Default|SetSubjectID (Math|Conversions|ToInteger(Byte) (Variables|Default|GetPatientID-Hardcode))))
      ;[1 1 1] These were connected.
      (Utilities|Array|AddUnique (Variables|Default|GetPatientList_Hardcoded) _output_get)
      (bind (_direction _confusion_line) (Default|TrivectorProtocol (Variables|Default|GetthisColorCamera) _device)))))

(event Input|EnhancedActionEvents|EnhancedInputActionPicoInputDown
  (params (ActionValue :type Boolean) (ElapsedSeconds :type Float%20%28double-precision%29) (TriggeredSeconds :type Float%20%28double-precision%29) (InputAction :type Input%20Action%20Object%20Reference :default "/Game/PicoInput/PicoInputDown.PicoInputDown"))
  (Default|ChangeOption (Variables|Default|Getui) false))

(event Input|EnhancedActionEvents|EnhancedInputActionPicoInputLeft
  (params (ActionValue :type Boolean) (ElapsedSeconds :type Float%20%28double-precision%29) (TriggeredSeconds :type Float%20%28double-precision%29) (InputAction :type Input%20Action%20Object%20Reference :default "/Game/PicoInput/PicoInputLeft.PicoInputLeft"))
  (Default|ChangeSelection (Variables|Default|Getui)))

(event Input|EnhancedActionEvents|EnhancedInputActionPicoInputRight
  (params (ActionValue :type Boolean) (ElapsedSeconds :type Float%20%28double-precision%29) (TriggeredSeconds :type Float%20%28double-precision%29) (InputAction :type Input%20Action%20Object%20Reference :default "/Game/PicoInput/PicoInputRight.PicoInputRight"))
  (Default|ChangeSelection (Variables|Default|Getui)))

(event Input|EnhancedActionEvents|EnhancedInputActionPicoInputUpR
  (params (ActionValue :type Boolean) (ElapsedSeconds :type Float%20%28double-precision%29) (TriggeredSeconds :type Float%20%28double-precision%29) (InputAction :type Input%20Action%20Object%20Reference :default "/Game/PicoInput/PicoInputUpR.PicoInputUpR"))
  (bind _global (Variables|Default|GetGlobal))
  (bind _thiscolorcamera (Variables|Default|GetthisColorCamera))
  (bind _savegame (Variables|/Game/CVDGlobal.CVDGlobal_C|GetsaveGame _global))
  (bind _cal_lib (Variables|/Script/RAPD.CalibratedCamera|Getcal_lib _thiscolorcamera))
  (Variables|Default|Setresponse 0)
  (if (Variables|Default|Getdone)
    (bind (_new_confusion_line _new_direction) (Class|ColorCalibration|TrivectorTestResponse _cal_lib (Variables|Default|Getresponse) (Variables|Default|Getorientation) (Variables|Default|Getconfusion_line)))
    (CallFunction|Unobscure)
    (CallFunction|CountStart)
    (Variables|Default|Setorientation _new_direction)
    (Variables|Default|Setconfusion_line _new_confusion_line)
    (if (Variables|/Script/RAPD.ColorCalibration|Getall_test_done _cal_lib)
      (Class|ColorCalibration|RecordResponsetoCSV _cal_lib (Utilities|String|ToString(Integer) (Variables|Default|GetsubjectID)))
      (Variables|/Game/SaveCVD.SaveCVD_C|Setdone _savegame false)
      (SaveGame|SaveGametoSlot _savegame "save")
      (Game|OpenLevel(byName) "ColorTest"))))

(event Input|EnhancedActionEvents|EnhancedInputActionPicoInputLeftR
  (params (ActionValue :type Boolean) (ElapsedSeconds :type Float%20%28double-precision%29) (TriggeredSeconds :type Float%20%28double-precision%29) (InputAction :type Input%20Action%20Object%20Reference :default "/Game/PicoInput/PicoInputLeftR.PicoInputLeftR"))
  (bind _global (Variables|Default|GetGlobal))
  (bind _thiscolorcamera (Variables|Default|GetthisColorCamera))
  (bind _savegame (Variables|/Game/CVDGlobal.CVDGlobal_C|GetsaveGame _global))
  (bind _cal_lib (Variables|/Script/RAPD.CalibratedCamera|Getcal_lib _thiscolorcamera))
  (Variables|Default|Setresponse 1)
  (if (Variables|Default|Getdone)
    (bind (_new_confusion_line _new_direction) (Class|ColorCalibration|TrivectorTestResponse _cal_lib (Variables|Default|Getresponse) (Variables|Default|Getorientation) (Variables|Default|Getconfusion_line)))
    (CallFunction|Unobscure)
    (CallFunction|CountStart)
    (Variables|Default|Setorientation _new_direction)
    (Variables|Default|Setconfusion_line _new_confusion_line)
    (if (Variables|/Script/RAPD.ColorCalibration|Getall_test_done _cal_lib)
      (Class|ColorCalibration|RecordResponsetoCSV _cal_lib (Utilities|String|ToString(Integer) (Variables|Default|GetsubjectID)))
      (Variables|/Game/SaveCVD.SaveCVD_C|Setdone _savegame false)
      (SaveGame|SaveGametoSlot _savegame "save")
      (Game|OpenLevel(byName) "ColorTest"))))

(event Input|EnhancedActionEvents|EnhancedInputActionPicoInputRightR
  (params (ActionValue :type Boolean) (ElapsedSeconds :type Float%20%28double-precision%29) (TriggeredSeconds :type Float%20%28double-precision%29) (InputAction :type Input%20Action%20Object%20Reference :default "/Game/PicoInput/PicoInputRightR.PicoInputRightR"))
  (bind _global (Variables|Default|GetGlobal))
  (bind _thiscolorcamera (Variables|Default|GetthisColorCamera))
  (bind _savegame (Variables|/Game/CVDGlobal.CVDGlobal_C|GetsaveGame _global))
  (bind _cal_lib (Variables|/Script/RAPD.CalibratedCamera|Getcal_lib _thiscolorcamera))
  (Variables|Default|Setresponse 3)
  (if (Variables|Default|Getdone)
    (bind (_new_confusion_line _new_direction) (Class|ColorCalibration|TrivectorTestResponse _cal_lib (Variables|Default|Getresponse) (Variables|Default|Getorientation) (Variables|Default|Getconfusion_line)))
    (CallFunction|Unobscure)
    (CallFunction|CountStart)
    (Variables|Default|Setorientation _new_direction)
    (Variables|Default|Setconfusion_line _new_confusion_line)
    (if (Variables|/Script/RAPD.ColorCalibration|Getall_test_done _cal_lib)
      (Class|ColorCalibration|RecordResponsetoCSV _cal_lib (Utilities|String|ToString(Integer) (Variables|Default|GetsubjectID)))
      (Variables|/Game/SaveCVD.SaveCVD_C|Setdone _savegame false)
      (SaveGame|SaveGametoSlot _savegame "save")
      (Game|OpenLevel(byName) "ColorTest"))))

(event Input|EnhancedActionEvents|EnhancedInputActionPicoInputDownR
  (params (ActionValue :type Boolean) (ElapsedSeconds :type Float%20%28double-precision%29) (TriggeredSeconds :type Float%20%28double-precision%29) (InputAction :type Input%20Action%20Object%20Reference :default "/Game/PicoInput/PicoInputDownR.PicoInputDownR"))
  (bind _global (Variables|Default|GetGlobal))
  (bind _thiscolorcamera (Variables|Default|GetthisColorCamera))
  (bind _savegame (Variables|/Game/CVDGlobal.CVDGlobal_C|GetsaveGame _global))
  (bind _cal_lib (Variables|/Script/RAPD.CalibratedCamera|Getcal_lib _thiscolorcamera))
  (Variables|Default|Setresponse 2)
  (if (Variables|Default|Getdone)
    (bind (_new_confusion_line _new_direction) (Class|ColorCalibration|TrivectorTestResponse _cal_lib (Variables|Default|Getresponse) (Variables|Default|Getorientation) (Variables|Default|Getconfusion_line)))
    (CallFunction|Unobscure)
    (CallFunction|CountStart)
    (Variables|Default|Setorientation _new_direction)
    (Variables|Default|Setconfusion_line _new_confusion_line)
    (if (Variables|/Script/RAPD.ColorCalibration|Getall_test_done _cal_lib)
      (Class|ColorCalibration|RecordResponsetoCSV _cal_lib (Utilities|String|ToString(Integer) (Variables|Default|GetsubjectID)))
      (Variables|/Game/SaveCVD.SaveCVD_C|Setdone _savegame false)
      (SaveGame|SaveGametoSlot _savegame "save")
      (Game|OpenLevel(byName) "ColorTest"))))

(event Input|EnhancedActionEvents|EnhancedInputActionPicoInputUp
  (params (ActionValue :type Boolean) (ElapsedSeconds :type Float%20%28double-precision%29) (TriggeredSeconds :type Float%20%28double-precision%29) (InputAction :type Input%20Action%20Object%20Reference :default "/Game/PicoInput/PicoInputUp.PicoInputUp"))
  (Default|ChangeOption (Variables|Default|Getui) true))

(event EventBeginPlay
  (bind _returnvalue (Game|GetPlayerController 0))
  (Input|AddMappingContext (PlayerController|LocalPlayerSubsystems|GetEnhancedInputLocalPlayerSubsystem _returnvalue) "/Game/PicoInput/PicoColor.PicoColor" 10 "(bIgnoreAllPressedKeysUntilRelease=True,bForceImmediately=False,bNotifyUserSettings=False)")
  (bind _ascolor_camera (Utilities|Casting|CastToColorCamera (Variables|/Script/Engine.ChildActorComponent|GetChildActor (Variables|Default|GetcolorCam))))
  (Variables|Default|SetthisColorCamera _ascolor_camera)
  (Development|PrintString "CAmera CAst OK")
  (Game|Player|SetViewTargetwithBlend _returnvalue (Variables|Default|GetthisColorCamera) 0.0 "VTBlend_Linear" 0.0 false)
  (Development|PrintString "View Blended")
  (Rendering|SetVisibility (Variables|/Game/Blueprints/ColorCamera.ColorCamera_C|GetCanvas (Variables|Default|GetthisColorCamera)) false true)
  (bind _ascolor_ui (Utilities|Casting|CastToColor_UI (UserInterface|GetUserWidgetObject (Variables|/Game/Blueprints/ColorCamera.ColorCamera_C|Getui (Variables|Default|GetthisColorCamera)))))
  (Development|PrintString "Cast to UI Succeeded," true true "(R=0.011616,G=1.000000,B=0.000374,A=1.000000)" 1e+01)
  ;[1 1 1] Connect these two.
  (bind _output_get (Variables|Default|Setui _ascolor_ui))
  (bind _ascvdglobal (Utilities|Casting|CastToCVDGlobal (Game|GetGameInstance))
    (:then
      (bind _output_get_2 (Variables|Default|SetGlobal _ascvdglobal))
      (Development|PrintString "Check.")
      (bind _returnvalue_2 (SaveGame|DoesSaveGameExist "saveCVD"))
      (Development|PrintString "Save Distance Check")
      (if _returnvalue_2
        (bind _returnvalue_3 (SaveGame|LoadGamefromSlot "saveCVD"))
        (bind _assave_cvd (Utilities|Casting|CastToSaveCVD _returnvalue_3))
        (Variables|/Game/CVDGlobal.CVDGlobal_C|SetsaveGame _output_get_2 _assave_cvd)
        (else
          (bind _returnvalue_4 (SaveGame|CreateSaveGameObject "/Game/SaveCVD.SaveCVD_C"))
          (Variables|/Game/CVDGlobal.CVDGlobal_C|SetsaveGame _output_get_2 _returnvalue_4)))
      (if (> (Utilities|Array|Length (Variables|/Game/SaveCVD.SaveCVD_C|Getpatient_list (Variables|/Game/CVDGlobal.CVDGlobal_C|GetsaveGame _output_get_2))) 0)
        (Utilities|FlowControl|DoOnce false
          (:Completed
            (Default|Neopopulate _output_get (Variables|/Game/SaveCVD.SaveCVD_C|Getpatient_list (Variables|/Game/CVDGlobal.CVDGlobal_C|GetsaveGame _output_get_2)))))))
    (:CastFailed
      (Development|PrintString "CAst to GlobalCVD failed." true true "(R=0.000000,G=0.660000,B=1.000000,A=1.000000)" 12.0))))

(event Collision|EventActorBeginOverlap
  (params (OtherActor :type Actor%20Object%20Reference)))

(event EventTick
  (params (DeltaSeconds :type Float%20%28single-precision%29))
  (bind _thiscolorcamera (Variables|Default|GetthisColorCamera))
  (bind _cal_lib (Variables|/Script/RAPD.CalibratedCamera|Getcal_lib _thiscolorcamera))
  (Variables|/Script/RAPD.ColorCalibration|Setcurrent_time _cal_lib (+ (Variables|/Script/RAPD.ColorCalibration|Getcurrent_time _cal_lib) DeltaSeconds)))

(event Input|KeyboardEvents|SpaceBar
  (params (Key :type Key%20Structure :default "None"))
  (bind _thiscolorcamera (Variables|Default|GetthisColorCamera))
  (:Pressed
    (Development|PrintString "Pico Triggered")
    (Utilities|FlowControl|DoOnce false
      (:Completed
        (Rendering|SetVisibility (Variables|/Game/Blueprints/ColorCamera.ColorCamera_C|Getui _thiscolorcamera) false true)
        (Rendering|SetVisibility (Variables|/Game/Blueprints/ColorCamera.ColorCamera_C|GetCanvas _thiscolorcamera) true true)
        ;[1 1 1] Connect These two
        (bind _device (Default|Selections (Variables|Default|Getui)))
        (bind _output_get (Variables|Default|SetSubjectID (Math|Conversions|ToInteger(Byte) (Variables|Default|GetPatientID-Hardcode))))
        ;[1 1 1] These were connected.
        (Utilities|Array|AddUnique (Variables|Default|GetPatientList_Hardcoded) _output_get)
        (bind (_direction _confusion_line) (Default|TrivectorProtocol (Variables|Default|GetthisColorCamera) _device))))))

(fn ConstructionScript)