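; Player pawn for eye assessments on Pico controller input, covering reading, static and dynamic visual acuity, and contrast sensitivity tests.
; It shows start and assessment widgets on a child AssessCamera, which runs the chosen test and moves the Dynamic VA stimulus on Tick.
; Directional inputs become Numpad trackpad responses that the camera scores and the pawn records.
; FlowAssess saves through the game instance, then switches monocular tests to the right eye or lets EyeTests reload.
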(event Custom|Place%20Start%20Widget
  (bind _returnvalue (Game|GetPlayerController 0))
  (bind _returnvalue_2 (PlayerController|LocalPlayerSubsystems|GetEnhancedInputLocalPlayerSubsystem _returnvalue))
  ;[1 1 1] Paces the Start Menu
  (bind _asassess_camera (Utilities|Casting|CastToAssessCamera (Variables|/Script/Engine.ChildActorComponent|GetChildActor (Variables|Default|Getcamera))))
  (bind _output_get (Variables|Default|SetCalCam _asassess_camera))
  (Game|Player|SetViewTargetwithBlend (Game|GetPlayerController 0) _output_get 0.0 "VTBlend_Linear" 0.0 false)
  (bind _returnvalue_3 (UserInterface|CreateWidget "/Game/UI/start_screen.start_screen_C"))
  (Variables|Default|SetstartWidget _returnvalue_3)
  (UserInterface|SetWidget (Variables|/Game/Blueprints/AssessCamera.AssessCamera_C|GetmyUI _output_get) _returnvalue_3)
  (Rendering|SetVisibility (Variables|/Game/Blueprints/AssessCamera.AssessCamera_C|GetmyUI _output_get) true true)
  (Input|EnableInput _returnvalue)
  (Class|EnhancedInputSubsystemInterface|ClearAllMappings _returnvalue_2)
  (Input|AddMappingContext _returnvalue_2 "/Game/PicoInput/PicoColor.PicoColor" 10 "(bIgnoreAllPressedKeysUntilRelease=True,bForceImmediately=False,bNotifyUserSettings=False)") ; Why using pico color for mapping context?
)

(event Input|EnhancedActionEvents|EnhancedInputActionPicoInputUpR
  (params (ActionValue :type Boolean) (ElapsedSeconds :type Float%20%28double-precision%29) (TriggeredSeconds :type Float%20%28double-precision%29) (InputAction :type Input%20Action%20Object%20Reference :default "/Game/PicoInput/PicoInputUpR.PicoInputUpR"))
  ;[1 1 1] Input controller translated to trackpad values for collecting responses
  (Utilities|VerifyStarted
    (:Ok
      (Default|Trackpad (Variables|Default|GetnumWidget) 0.0 1.0)
      (Class|SubjectPawn|SelectedResponse)
      (Development|PrintString "Selected response/"))))

(event Input|EnhancedActionEvents|EnhancedInputActionPicoInputDownR
  (params (ActionValue :type Boolean) (ElapsedSeconds :type Float%20%28double-precision%29) (TriggeredSeconds :type Float%20%28double-precision%29) (InputAction :type Input%20Action%20Object%20Reference :default "/Game/PicoInput/PicoInputDownR.PicoInputDownR"))
  ;[1 1 1] Input controller translated to trackpad values for collecting responses
  (Utilities|VerifyStarted
    (:Ok
      (Default|Trackpad (Variables|Default|GetnumWidget) 0.0 -1.0)
      (Class|SubjectPawn|SelectedResponse)
      (Development|PrintString "Selected response/"))))

(event Input|EnhancedActionEvents|EnhancedInputActionPicoInputLeft
  (params (ActionValue :type Boolean) (ElapsedSeconds :type Float%20%28double-precision%29) (TriggeredSeconds :type Float%20%28double-precision%29) (InputAction :type Input%20Action%20Object%20Reference :default "/Game/PicoInput/PicoInputLeft.PicoInputLeft"))
  ;[1 1 1] This is to move focus on (test/subject ID)
  (Default|ChangeOption (Variables|Default|GetstartWidget) false))

(event Input|EnhancedActionEvents|EnhancedInputActionPicoInputRight
  (params (ActionValue :type Boolean) (ElapsedSeconds :type Float%20%28double-precision%29) (TriggeredSeconds :type Float%20%28double-precision%29) (InputAction :type Input%20Action%20Object%20Reference :default "/Game/PicoInput/PicoInputRight.PicoInputRight"))
  ;[1 1 1] This is to move focus on (test/subject ID)
  (Default|ChangeOption (Variables|Default|GetstartWidget) true))

(event Input|EnhancedActionEvents|EnhancedInputActionPicoInputStore
  (params (ActionValue :type Boolean) (ElapsedSeconds :type Float%20%28double-precision%29) (TriggeredSeconds :type Float%20%28double-precision%29) (InputAction :type Input%20Action%20Object%20Reference :default "/Game/PicoInput/PicoInputStore.PicoInputStore")))

(event Input|EnhancedActionEvents|EnhancedInputActionPicoInputEnter
  (params (ActionValue :type Boolean) (ElapsedSeconds :type Float%20%28double-precision%29) (TriggeredSeconds :type Float%20%28double-precision%29) (InputAction :type Input%20Action%20Object%20Reference :default "/Game/PicoInput/PicoInputEnter.PicoInputEnter"))
  ;[1 1 1] Start selected test.
  (if (Variables|Default|Getstarted)
    (Game|OpenLevel(byName) "EyeTests")
    (else
      (Class|SubjectPawn|SelectedAssessment))))

(event Input|EnhancedActionEvents|EnhancedInputActionPicoInputUp
  (params (ActionValue :type Boolean) (ElapsedSeconds :type Float%20%28double-precision%29) (TriggeredSeconds :type Float%20%28double-precision%29) (InputAction :type Input%20Action%20Object%20Reference :default "/Game/PicoInput/PicoInputUp.PicoInputUp"))
  ;[1 1 1] Up-Down Selection (Test and Subject ID)
  (Default|UpDownSelection (Variables|Default|GetstartWidget)))

(event Input|EnhancedActionEvents|EnhancedInputActionPicoInputDown
  (params (ActionValue :type Boolean) (ElapsedSeconds :type Float%20%28double-precision%29) (TriggeredSeconds :type Float%20%28double-precision%29) (InputAction :type Input%20Action%20Object%20Reference :default "/Game/PicoInput/PicoInputDown.PicoInputDown"))
  ;[1 1 1] Up-Down Selection (Test and Subject ID)
  (Default|UpDownSelection (Variables|Default|GetstartWidget)))

(event Input|EnhancedActionEvents|EnhancedInputActionPicoInputLeftR
  (params (ActionValue :type Boolean) (ElapsedSeconds :type Float%20%28double-precision%29) (TriggeredSeconds :type Float%20%28double-precision%29) (InputAction :type Input%20Action%20Object%20Reference :default "/Game/PicoInput/PicoInputLeftR.PicoInputLeftR"))
  ;[1 1 1] Input controller translated to trackpad values for collecting responses
  (Utilities|VerifyStarted
    (:Ok
      (Default|Trackpad (Variables|Default|GetnumWidget) -1.0 0.0)
      (Class|SubjectPawn|SelectedResponse)
      (Development|PrintString "Selected response/"))))

(event Input|EnhancedActionEvents|EnhancedInputActionPicoInputRightR
  (params (ActionValue :type Boolean) (ElapsedSeconds :type Float%20%28double-precision%29) (TriggeredSeconds :type Float%20%28double-precision%29) (InputAction :type Input%20Action%20Object%20Reference :default "/Game/PicoInput/PicoInputRightR.PicoInputRightR"))
  ;[1 1 1] Input controller translated to trackpad values for collecting responses
  (Utilities|VerifyStarted
    (:Ok
      (Default|Trackpad (Variables|Default|GetnumWidget) 1.0 0.0)
      (Class|SubjectPawn|SelectedResponse)
      (Development|PrintString "Selected response/"))))

(event EventBeginPlay
  ;[1 1 1] Event-BeginPLay: Sets up enhanced input, cast the game instance into Visual Function Global game instance.
  (Input|AddMappingContext (PlayerController|LocalPlayerSubsystems|GetEnhancedInputLocalPlayerSubsystem (Game|GetPlayerController 0)) 0 10 "(bIgnoreAllPressedKeysUntilRelease=True,bForceImmediately=False,bNotifyUserSettings=False)")
  (Utilities|Casting|CastToVisual_Function_Global (Game|GetGameInstance)
    (:then
      (CallFunction|PlaceStartWidget))
    (:CastFailed
      (Development|PrintString "Cast Failed."))))

(event EventTick
  (params (DeltaSeconds :type Float%20%28single-precision%29))
  ;[1 1 1] If Dynamic VA - move stimulus
  (if (Variables|Default|Getstarted)
    (switch string (Variables|/Game/UI/UI_Assess.UI_Assess_C|GetWhich_test (Variables|Default|GetassessWidget))
      (:Dynamic%20VA
        (bind _new_direction (Class|EyeCamera|MovePointer (Variables|Default|GetCalCam) (Variables|Default|Getdirection) 0.0))
        (Variables|Default|Setdirection _new_direction)))))

(event EventSelectedAssessment
  (bind _calcam (Variables|Default|GetCalCam))
  (bind _calcam_2 (Variables|Default|GetCalCam))
  (bind _startwidget (Variables|Default|GetstartWidget))
  ;[1 1 1] Set up the Selected Test: Remove start screen widget, add numpad (if needed), set boolean for starting test and create test widgets.
  (bind (_test _subjectid) (Default|StartTest _startwidget))
  (Variables|Default|SetCurrentDesired%20Test%20Type _test)
  (Variables|Default|SetsubjectID _subjectid)
  (Widget|RemovefromParent _startwidget)
  (bind _asnumpad (Utilities|Casting|CastToNumpad (UserInterface|GetWidget (Variables|Default|Getnumpad))))
  (Variables|Default|SetnumWidget _asnumpad)
  (Variables|Default|Setstarted true)
  (bind _returnvalue (UserInterface|CreateWidget "/Game/UI/UI_Assess.UI_Assess_C"))
  (Variables|Default|SetassessWidget _returnvalue)
  (UserInterface|SetWidget (Variables|/Game/Blueprints/AssessCamera.AssessCamera_C|GetmyUI (Variables|Default|GetCalCam)) _returnvalue)
  (Default|SelectedTest _returnvalue (Variables|Default|GetCurrentDesired%20Test%20Type))
  (switch string (Variables|Default|GetCurrentDesired%20Test%20Type)
    (:Reading%20Test
      (Class|EyeCamera|ReadingTest _calcam_2)
      (Variables|/Script/RAPD.EyeCamera|Setcurrent_orientation_C _calcam 2)
      (Variables|/Script/RAPD.EyeCamera|Setprevious_orientation_C _calcam 2))
    (:Static%20VA%20Bino
      (Class|EyeCamera|BinocularStatic _calcam_2)
      (Variables|/Script/RAPD.EyeCamera|Setcurrent_orientation_C _calcam 0 :!label _label)
      (Variables|/Script/RAPD.EyeCamera|Setprevious_orientation_C _calcam 0))
    (:Static%20VA%20Mono
      (Class|EyeCamera|MonocularLeft _calcam_2)
      (goto _label))
    (:Dynamic%20VA
      (Variables|Default|Setdirection "0.000000,1.000000,0.000000")
      (Class|EyeCamera|BinocularDynamic _calcam_2)
      (goto _label))
    (:CS%20Mono
      (Class|EyeCamera|CS _calcam_2)
      (goto _label))))

(event EventSelectedResponse
  (bind _calcam (Variables|Default|GetCalCam))
  (bind _previous_orientation_c (Variables|/Script/RAPD.EyeCamera|Getprevious_orientation_C _calcam))
  (bind _recent_right_c (Variables|/Script/RAPD.EyeCamera|Getrecent_right_C _calcam))
  ;[1 1 1] Run selected test and compare responses to correct stimulus.
  (if (Variables|Default|Getstarted)
    (bind _completed (Class|EyeCamera|AssessResponses _calcam (Variables|/Game/UI/Numpad.Numpad_C|Getoutput (Variables|Default|GetnumWidget)) (Variables|/Game/UI/UI_Assess.UI_Assess_C|GetWhich_test (Variables|Default|GetassessWidget))))
    (if _completed
      (bind _result (Class|EyeCamera|ObtainResults (Variables|Default|GetCalCam) (Variables|/Game/UI/UI_Assess.UI_Assess_C|GetWhich_test (Variables|Default|GetassessWidget))))
      (bind _done (Class|SubjectPawn|FlowAssess))
      (Class|SubjectPawn|WritePatientRecord (Variables|/Game/UI/UI_Assess.UI_Assess_C|GetWhich_test (Variables|Default|GetassessWidget)) _result (not _done))
      (if _done
        (Game|OpenLevel(byName) "EyeTests"))
      (else
        (bind _time (Default|GetTime (Variables|Default|GetassessWidget)))
        (Class|SubjectPawn|RecordResponse (Math|Timespan|GetTotalSeconds _time) (Variables|/Script/RAPD.EyeCamera|Getwhich_eye_C _calcam) (Utilities|Array|Get(acopy) (Variables|Default|Getdirect) _previous_orientation_c) (Variables|/Game/UI/Numpad.Numpad_C|Getoutput (Variables|Default|GetnumWidget)) _recent_right_c (Variables|/Script/RAPD.EyeCamera|Getcurrent_log_C _calcam))
        (Default|Orientation (Variables|Default|GetassessWidget) _previous_orientation_c _recent_right_c)))))

(event Input|KeyboardEvents|S
  (params (Key :type Key%20Structure :default "None"))
  ;[1 1 1] Up-Down Selection (Test and Subject ID)
  (:Pressed
    (Default|UpDownSelection (Variables|Default|GetstartWidget))))

(event Input|KeyboardEvents|W
  (params (Key :type Key%20Structure :default "None"))
  ;[1 1 1] Up-Down Selection (Test and Subject ID)
  (:Pressed
    (Default|UpDownSelection (Variables|Default|GetstartWidget))))

(event Input|KeyboardEvents|Up
  (params (Key :type Key%20Structure :default "None")))

(event Input|KeyboardEvents|Down
  (params (Key :type Key%20Structure :default "None")))

(event Input|KeyboardEvents|Left
  (params (Key :type Key%20Structure :default "None"))
  ;[1 1 1] This is to move focus on (test/subject ID)
)

(event Input|KeyboardEvents|Right
  (params (Key :type Key%20Structure :default "None"))
  ;[1 1 1] This is to move focus on (test/subject ID)
)

(fn ConstructionScript)

(fn FlowAssess
  (bind _calcam (Variables|Default|GetCalCam))
  (bind _which_eye_c (Variables|/Script/RAPD.EyeCamera|Getwhich_eye_C _calcam))
  (bind _asvisual_function_global (Utilities|Casting|CastToVisual_Function_Global (Game|GetGameInstance)))
  (Default|AddNewPatient _asvisual_function_global (Variables|Default|GetsubjectID))
  (Default|WritetoSaveGame _asvisual_function_global false)
  (switch string (Variables|/Game/UI/UI_Assess.UI_Assess_C|GetWhich_test (Variables|Default|GetassessWidget))
    (:Default
      _)
    (:CS%20Mono
      (switch string _which_eye_c
        (:Left
          (Class|EyeCamera|CSRight _calcam)
          (Variables|/Script/RAPD.EyeCamera|Setcurrent_orientation_C _calcam 0 :!label _label)
          (Variables|/Script/RAPD.EyeCamera|Setprevious_orientation_C _calcam 0)
          (return false))
        (:Right
          _)))
    (:Static%20VA%20Mono
      (switch string _which_eye_c
        (:Left
          (Class|EyeCamera|MonocularRight _calcam)
          (goto _label))
        (:Right
          _))))
  (return true))