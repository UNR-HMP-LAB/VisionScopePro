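; Global patient data store for a visual function testing app, covering static and dynamic acuity, contrast sensitivity and scotoma/metamorphopsia parameters.
; StartUp loads AllPatients from the "Patient Info" save slot; WriteToSaveGame drops assessments without valid results, optionally clears all, then saves.
; Add functions look patients up by ID and write into their latest assessment, flagging that test valid.
; Scotoma parameters are staged in TempMeta for recall or committing via VisitedMeta.
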(fn PatientExists
  (params (ID :type Integer))
  (for (_array_element _array_index) (Variables|Patient_Data|Getall_patients)
    (if (== (.id _array_element) ID)
      (return (Class|KismetSystemLibrary|MakeLiteralBool true) _array_index)))
  (return (Class|KismetSystemLibrary|MakeLiteralBool false) -1))

(fn WritetoSaveGame
  (params (delete :type Boolean))
  (bind _temp (Variables|Patient_Data|Gettemp))
  (bind _all_patients (Variables|Patient_Data|Getall_patients))
  (bind _returnvalue (SaveGame|CreateSaveGameObject "/Game/Blueprints/Visual_Function_Save.Visual_Function_Save_C"))
  (for (_array_element _array_index) _all_patients
    (for (_array_element_2 _array_index_2) (.assessments _array_element)
      (if (Math|Boolean|ORBoolean (.static_va_valid _array_element_2) (.dynamic_va_valid _array_element_2) (.cs_valid _array_element_2) (.scotoma_parameters_valid _array_element_2))
        (Utilities|Array|Add _temp (Utilities|Array|Get(acopy) (.assessments _array_element) _array_index_2))))
    (Utilities|Array|SetArrayElem _all_patients _array_index (Utilities|Struct|MakePatient (.id _array_element) _temp))
    (Utilities|Array|Clear _temp))
  (if delete
    (Utilities|Array|Clear _all_patients))
  (Variables|/Game/Blueprints/Visual_Function_Save.Visual_Function_Save_C|SetPatient%20Info _returnvalue _all_patients)
  (SaveGame|SaveGametoSlot _returnvalue "Patient Info"))

(fn StartUp
  (bind _returnvalue (SaveGame|DoesSaveGameExist "Patient Info"))
  (if _returnvalue
    (bind _returnvalue_2 (SaveGame|LoadGamefromSlot "Patient Info"))
    (bind _asvisual_function_save (Utilities|Casting|CastToVisual_Function_Save _returnvalue_2))
    (Variables|Patient_Data|Setall_patients (Variables|/Game/Blueprints/Visual_Function_Save.Visual_Function_Save_C|GetPatient%20Info _asvisual_function_save))
    (else
      (bind _returnvalue_3 (SaveGame|CreateSaveGameObject "/Game/Blueprints/Visual_Function_Save.Visual_Function_Save_C"))
      (Variables|Patient_Data|Setall_patients (Variables|/Game/Blueprints/Visual_Function_Save.Visual_Function_Save_C|GetPatient%20Info _returnvalue_3)))))

(fn AddNewAssessment
  (params (patient_ID :type Integer))
  (bind _index (CallFunction|PatientExists patient_ID))
  (bind _returnvalue (Utilities|Array|Add (.assessments (Utilities|Array|Get(acopy) (Variables|Patient_Data|Getall_patients) _index)) (Utilities|Struct|Makepatient_assessment false false false false (Utilities|Map|MakeMap "" 0.0) 0.0 0 (Utilities|Array|MakeArray "") (Math|DateTime|Now))))
  (return _returnvalue))

(fn AddNewPatient
  (params (patient_ID :type Integer) (Name :type String) (Age :type Integer) (Sex :type String))
  (bind _all_patients (Variables|Patient_Data|Getall_patients))
  (bind _exists (CallFunction|PatientExists patient_ID))
  (if (not _exists)
    (bind _returnvalue (Utilities|Array|Add _all_patients (Utilities|Struct|MakePatient patient_ID (Utilities|Array|MakeArray ""))))
    (Utilities|Array|RemoveIndex (.assessments (Utilities|Array|Get(acopy) _all_patients _returnvalue)))))

(fn AddStaticVA
  (params (whichEye :type String) (patient_ID :type Integer) (logMAR :type Float%20%28double-precision%29))
  (bind (_exists _index) (CallFunction|PatientExists patient_ID))
  (if _exists
    (Utilities|Map|Add (.static_va (Utilities|Array|Get(acopy) (.assessments (Utilities|Array|Get(acopy) (Variables|Patient_Data|Getall_patients) _index)) (Utilities|Array|LastIndex (.assessments (Utilities|Array|Get(acopy) (Variables|Patient_Data|Getall_patients) _index))))) whichEye logMAR)
    (Utilities|Array|SetArrayElem (.assessments (Utilities|Array|Get(acopy) (Variables|Patient_Data|Getall_patients) _index)) (Utilities|Array|LastIndex (.assessments (Utilities|Array|Get(acopy) (Variables|Patient_Data|Getall_patients) _index))) (Utilities|Struct|Makepatient_assessment true (.dynamic_va_valid (Utilities|Array|Get(acopy) (.assessments (Utilities|Array|Get(acopy) (Variables|Patient_Data|Getall_patients) _index)) (Utilities|Array|LastIndex (.assessments (Utilities|Array|Get(acopy) (Variables|Patient_Data|Getall_patients) _index))))) (.cs_valid (Utilities|Array|Get(acopy) (.assessments (Utilities|Array|Get(acopy) (Variables|Patient_Data|Getall_patients) _index)) (Utilities|Array|LastIndex (.assessments (Utilities|Array|Get(acopy) (Variables|Patient_Data|Getall_patients) _index))))) (.scotoma_parameters_valid (Utilities|Array|Get(acopy) (.assessments (Utilities|Array|Get(acopy) (Variables|Patient_Data|Getall_patients) _index)) (Utilities|Array|LastIndex (.assessments (Utilities|Array|Get(acopy) (Variables|Patient_Data|Getall_patients) _index))))) (.static_va (Utilities|Array|Get(acopy) (.assessments (Utilities|Array|Get(acopy) (Variables|Patient_Data|Getall_patients) _index)) (Utilities|Array|LastIndex (.assessments (Utilities|Array|Get(acopy) (Variables|Patient_Data|Getall_patients) _index))))) (.dynamic_va (Utilities|Array|Get(acopy) (.assessments (Utilities|Array|Get(acopy) (Variables|Patient_Data|Getall_patients) _index)) (Utilities|Array|LastIndex (.assessments (Utilities|Array|Get(acopy) (Variables|Patient_Data|Getall_patients) _index))))) (.cs (Utilities|Array|Get(acopy) (.assessments (Utilities|Array|Get(acopy) (Variables|Patient_Data|Getall_patients) _index)) (Utilities|Array|LastIndex (.assessments (Utilities|Array|Get(acopy) (Variables|Patient_Data|Getall_patients) _index))))) (.scotoma_parameters (Utilities|Array|Get(acopy) (.assessments (Utilities|Array|Get(acopy) (Variables|Patient_Data|Getall_patients) _index)) (Utilities|Array|LastIndex (.assessments (Utilities|Array|Get(acopy) (Variables|Patient_Data|Getall_patients) _index))))) (.time (Utilities|Array|Get(acopy) (.assessments (Utilities|Array|Get(acopy) (Variables|Patient_Data|Getall_patients) _index)) (Utilities|Array|LastIndex (.assessments (Utilities|Array|Get(acopy) (Variables|Patient_Data|Getall_patients) _index)))))))))

(fn AddDynamicVA
  (params (patient_ID :type Integer) (logMAR :type Float%20%28double-precision%29))
  (bind (_exists _index) (CallFunction|PatientExists patient_ID))
  (if _exists
    (Utilities|Array|SetArrayElem (.assessments (Utilities|Array|Get(acopy) (Variables|Patient_Data|Getall_patients) _index)) (Utilities|Array|LastIndex (.assessments (Utilities|Array|Get(acopy) (Variables|Patient_Data|Getall_patients) _index))) (Utilities|Struct|Makepatient_assessment (.static_va_valid (Utilities|Array|Get(acopy) (.assessments (Utilities|Array|Get(acopy) (Variables|Patient_Data|Getall_patients) _index)) (Utilities|Array|LastIndex (.assessments (Utilities|Array|Get(acopy) (Variables|Patient_Data|Getall_patients) _index))))) true (.cs_valid (Utilities|Array|Get(acopy) (.assessments (Utilities|Array|Get(acopy) (Variables|Patient_Data|Getall_patients) _index)) (Utilities|Array|LastIndex (.assessments (Utilities|Array|Get(acopy) (Variables|Patient_Data|Getall_patients) _index))))) (.scotoma_parameters_valid (Utilities|Array|Get(acopy) (.assessments (Utilities|Array|Get(acopy) (Variables|Patient_Data|Getall_patients) _index)) (Utilities|Array|LastIndex (.assessments (Utilities|Array|Get(acopy) (Variables|Patient_Data|Getall_patients) _index))))) (.static_va (Utilities|Array|Get(acopy) (.assessments (Utilities|Array|Get(acopy) (Variables|Patient_Data|Getall_patients) _index)) (Utilities|Array|LastIndex (.assessments (Utilities|Array|Get(acopy) (Variables|Patient_Data|Getall_patients) _index))))) logMAR (.cs (Utilities|Array|Get(acopy) (.assessments (Utilities|Array|Get(acopy) (Variables|Patient_Data|Getall_patients) _index)) (Utilities|Array|LastIndex (.assessments (Utilities|Array|Get(acopy) (Variables|Patient_Data|Getall_patients) _index))))) (.scotoma_parameters (Utilities|Array|Get(acopy) (.assessments (Utilities|Array|Get(acopy) (Variables|Patient_Data|Getall_patients) _index)) (Utilities|Array|LastIndex (.assessments (Utilities|Array|Get(acopy) (Variables|Patient_Data|Getall_patients) _index))))) (.time (Utilities|Array|Get(acopy) (.assessments (Utilities|Array|Get(acopy) (Variables|Patient_Data|Getall_patients) _index)) (Utilities|Array|LastIndex (.assessments (Utilities|Array|Get(acopy) (Variables|Patient_Data|Getall_patients) _index)))))))))

(fn AddCS
  (params (patient_ID :type Integer) (logCS :type Float%20%28double-precision%29) (Which_Eye :type String))
  (bind (_exists _index) (CallFunction|PatientExists patient_ID))
  (if _exists
    (Utilities|Map|Add (.cs (Utilities|Array|Get(acopy) (.assessments (Utilities|Array|Get(acopy) (Variables|Patient_Data|Getall_patients) _index)) (Utilities|Array|LastIndex (.assessments (Utilities|Array|Get(acopy) (Variables|Patient_Data|Getall_patients) _index))))) Which_Eye logCS)
    (Utilities|Array|SetArrayElem (.assessments (Utilities|Array|Get(acopy) (Variables|Patient_Data|Getall_patients) _index)) (Utilities|Array|LastIndex (.assessments (Utilities|Array|Get(acopy) (Variables|Patient_Data|Getall_patients) _index))) (Utilities|Struct|Makepatient_assessment (.static_va_valid (Utilities|Array|Get(acopy) (.assessments (Utilities|Array|Get(acopy) (Variables|Patient_Data|Getall_patients) _index)) (Utilities|Array|LastIndex (.assessments (Utilities|Array|Get(acopy) (Variables|Patient_Data|Getall_patients) _index))))) (.dynamic_va_valid (Utilities|Array|Get(acopy) (.assessments (Utilities|Array|Get(acopy) (Variables|Patient_Data|Getall_patients) _index)) (Utilities|Array|LastIndex (.assessments (Utilities|Array|Get(acopy) (Variables|Patient_Data|Getall_patients) _index))))) true (.scotoma_parameters_valid (Utilities|Array|Get(acopy) (.assessments (Utilities|Array|Get(acopy) (Variables|Patient_Data|Getall_patients) _index)) (Utilities|Array|LastIndex (.assessments (Utilities|Array|Get(acopy) (Variables|Patient_Data|Getall_patients) _index))))) (.static_va (Utilities|Array|Get(acopy) (.assessments (Utilities|Array|Get(acopy) (Variables|Patient_Data|Getall_patients) _index)) (Utilities|Array|LastIndex (.assessments (Utilities|Array|Get(acopy) (Variables|Patient_Data|Getall_patients) _index))))) (.dynamic_va (Utilities|Array|Get(acopy) (.assessments (Utilities|Array|Get(acopy) (Variables|Patient_Data|Getall_patients) _index)) (Utilities|Array|LastIndex (.assessments (Utilities|Array|Get(acopy) (Variables|Patient_Data|Getall_patients) _index))))) (.cs (Utilities|Array|Get(acopy) (.assessments (Utilities|Array|Get(acopy) (Variables|Patient_Data|Getall_patients) _index)) (Utilities|Array|LastIndex (.assessments (Utilities|Array|Get(acopy) (Variables|Patient_Data|Getall_patients) _index))))) (.scotoma_parameters (Utilities|Array|Get(acopy) (.assessments (Utilities|Array|Get(acopy) (Variables|Patient_Data|Getall_patients) _index)) (Utilities|Array|LastIndex (.assessments (Utilities|Array|Get(acopy) (Variables|Patient_Data|Getall_patients) _index))))) (.time (Utilities|Array|Get(acopy) (.assessments (Utilities|Array|Get(acopy) (Variables|Patient_Data|Getall_patients) _index)) (Utilities|Array|LastIndex (.assessments (Utilities|Array|Get(acopy) (Variables|Patient_Data|Getall_patients) _index)))))))))

(fn AddMetamorphopsia
  (bind _temp_meta (Variables|Patient_Data|Gettemp_meta))
  (if (Variables|Patient_Data|Getvisited_meta)
    (bind _index (CallFunction|PatientExists (Variables|PatientData|Gettemp_ID)))
    (Utilities|Array|SetArrayElem (.assessments (Utilities|Array|Get(acopy) (Variables|Patient_Data|Getall_patients) _index)) (Utilities|Array|LastIndex (.assessments (Utilities|Array|Get(acopy) (Variables|Patient_Data|Getall_patients) _index))) (Utilities|Struct|Makepatient_assessment (.static_va_valid (Utilities|Array|Get(acopy) (.assessments (Utilities|Array|Get(acopy) (Variables|Patient_Data|Getall_patients) _index)) (Utilities|Array|LastIndex (.assessments (Utilities|Array|Get(acopy) (Variables|Patient_Data|Getall_patients) _index))))) (.dynamic_va_valid (Utilities|Array|Get(acopy) (.assessments (Utilities|Array|Get(acopy) (Variables|Patient_Data|Getall_patients) _index)) (Utilities|Array|LastIndex (.assessments (Utilities|Array|Get(acopy) (Variables|Patient_Data|Getall_patients) _index))))) (.cs_valid (Utilities|Array|Get(acopy) (.assessments (Utilities|Array|Get(acopy) (Variables|Patient_Data|Getall_patients) _index)) (Utilities|Array|LastIndex (.assessments (Utilities|Array|Get(acopy) (Variables|Patient_Data|Getall_patients) _index))))) true (.static_va (Utilities|Array|Get(acopy) (.assessments (Utilities|Array|Get(acopy) (Variables|Patient_Data|Getall_patients) _index)) (Utilities|Array|LastIndex (.assessments (Utilities|Array|Get(acopy) (Variables|Patient_Data|Getall_patients) _index))))) (.dynamic_va (Utilities|Array|Get(acopy) (.assessments (Utilities|Array|Get(acopy) (Variables|Patient_Data|Getall_patients) _index)) (Utilities|Array|LastIndex (.assessments (Utilities|Array|Get(acopy) (Variables|Patient_Data|Getall_patients) _index))))) (.cs (Utilities|Array|Get(acopy) (.assessments (Utilities|Array|Get(acopy) (Variables|Patient_Data|Getall_patients) _index)) (Utilities|Array|LastIndex (.assessments (Utilities|Array|Get(acopy) (Variables|Patient_Data|Getall_patients) _index))))) _temp_meta (.time (Utilities|Array|Get(acopy) (.assessments (Utilities|Array|Get(acopy) (Variables|Patient_Data|Getall_patients) _index)) (Utilities|Array|LastIndex (.assessments (Utilities|Array|Get(acopy) (Variables|Patient_Data|Getall_patients) _index)))))))
    (Utilities|Array|Clear _temp_meta)
    (Variables|Patient_Data|Setvisited_meta false)))

(fn ExamplePatientData
  (params (patient_ID :type Integer))
  (bind _index (CallFunction|PatientExists patient_ID))
  (Utilities|Array|Add (.assessments (Utilities|Array|Get(acopy) (Variables|Patient_Data|Getall_patients) _index)) (Utilities|Struct|Makepatient_assessment true true true true (Utilities|Map|MakeMap "Left" 0.1 "Right" 0.1 "Binocular" 0.1) 0.2 (Utilities|Map|MakeMap "Left" 2.0 "Right" 2.0) (Utilities|Array|MakeArray (Utilities|Struct|MakeScotoma "(R=0.500000,G=0.500000,B=0.000000,A=0.000000)" 0.1 0.1 1e+01 1e+02 0.15)) (Math|DateTime|Now))))

(fn SendPatientPerception
  (params (patient_ID :type Integer) (session_ID :type Integer))
  (bind (_exists _index) (CallFunction|PatientExists patient_ID))
  (if _exists
    (Variables|Patient_Data|Settemp_meta (.scotoma_parameters (Utilities|Array|Get(acopy) (.assessments (Utilities|Array|Get(acopy) (Variables|Patient_Data|Getall_patients) _index)) session_ID)))
    (Variables|Patient_Data|Setvisited_meta (.scotoma_parameters_valid (Utilities|Array|Get(acopy) (.assessments (Utilities|Array|Get(acopy) (Variables|Patient_Data|Getall_patients) _index)) session_ID)))
    (return)))

(fn InitializeScotoma
  (bind _sigma (Variables|PatientData|Getsigma))
  (bind _rotation (Variables|PatientData|Getrotation))
  (bind _distortion (Variables|Patient_Data|Getdistortion))
  (Variables|Patient_Data|Settemp_meta (Utilities|Array|MakeArray (Utilities|Struct|MakeScotoma "(R=0.530000,G=0.500000,B=0.000000,A=0.000000)" _sigma 0.0 _rotation _distortion 0.15) (Utilities|Struct|MakeScotoma "(R=0.520000,G=0.500000,B=0.000000,A=0.000000)" _sigma 0.0 _rotation _distortion 0.15) (Utilities|Struct|MakeScotoma "(R=0.530000,G=0.550000,B=0.000000,A=0.000000)" _sigma 0.0 _rotation _distortion 0.15) (Utilities|Struct|MakeScotoma "(R=0.530000,G=0.450000,B=0.000000,A=0.000000)" _sigma 0.0 _rotation _distortion 0.15) (Utilities|Struct|MakeScotoma "(R=0.600000,G=0.500000,B=0.000000,A=0.000000)" _sigma 0.0 _rotation _distortion 0.15) (Utilities|Struct|MakeScotoma "(R=0.450000,G=0.500000,B=0.000000,A=0.000000)" _sigma 0.0 _rotation _distortion 0.15))))

(fn GetCurrentType
  (bind _pids (Variables|Default|GetPIDs))
  (bind (_id _pass _type) (Utilities|Struct|BreakPID _pids))
  (return _type _id))